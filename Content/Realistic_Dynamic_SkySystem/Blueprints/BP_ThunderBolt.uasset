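; Thunderbolt actor for the Realistic Dynamic Sky System that plays a one-shot lightning particle effect.
; BeginPlay randomizes the particle template and material, binds Fire to the FireLightning dispatcher and caches the sky Blueprint.
; Fire starts a fast looping timer that, when Loop is true, activates the particle and destroys the actor after a short random delay.
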(event `LightningEvent`
  ;[1 1 1] LightingBoltFire
  (if (`self.Loop`)
    (`ActorComponent.Activate` (`self.ThunderParticle`) false)
    (`KismetSystemLibrary.Delay` (`KismetMathLibrary.RandomFloatInRange` 1.0 2.0))
    (`self.K2_DestroyActor`)))

(event `Fire`
  (bind _timer (`self.Timer`))
  ;[1 1 1] Controls
  (bind _returnvalue (`KismetSystemLibrary.K2_SetTimerDelegate` (delegate `LightningEvent`) 0.008 true))
  (set `self.Timer` _returnvalue)
  (if (`KismetSystemLibrary.K2_IsTimerPausedHandle` _timer)
    (`KismetSystemLibrary.K2_UnPauseTimerHandle` _timer)))

(event `self.ReceiveBeginPlay`
  ;[1 1 1] Begin
  (`ParticleSystemComponent.SetTemplate` (`self.ThunderParticle`) (`|GetArrayItem` (`self.LightingBoltsParticles`) (`KismetMathLibrary.RandomIntegerInRange` 0 4)))
  (`PrimitiveComponent.SetMaterial` (`self.ThunderParticle`) 0 (`|GetArrayItem` (`self.LightingMaterials`) (`KismetMathLibrary.RandomIntegerInRange` 0 4)))
  (add `self.FireLightning` (delegate `Fire`))
  (bind _outactors (`GameplayStatics.GetAllActorsOfClass` "/Game/Realistic_Dynamic_SkySystem/Blueprints/RDS_Sky_BP.RDS_Sky_BP_C"))
  (set `self.BP_RDS` (`|GetArrayItem` _outactors)))

(fn `UserConstructionScript`)