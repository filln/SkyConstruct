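; Aurora controller for the SkyConstruct sky system that switches the aurora on and off and animates its look through the MPC_Aurora parameter collection.
; A looping timer on the owning BP_SkyConstructMain's clock rolls a weighted chance at one random hour per calendar window, then runs for a random real-time duration.
; In Interpolate mode, randomly chosen parameters ping-pong between min and max on a second timer.
; Manual modes allow direct toggling and live tuning.
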(event `self.ReceiveBeginPlay`
  (bind _asbp_skyconstructmain (cast `/Game/SkyConstruct/Blueprints/BP_SkyConstructMain` (`self.GetOwner`))
    (:`then`
      (set `self.BP_SkyConstructMain` _asbp_skyconstructmain)
      (`KismetSystemLibrary.K2_SetTimer` null "AuroraControl" (`self.AuroraControlDeltaTime`) true))
    (:`CastFailed`
      (`KismetSystemLibrary.PrintString` "BP_SkyConstructMain CastFailed"))))

(fn `AuroraControl`
  (if (`self.IsManualControl`)
    (`self.VariablesControl` (`self.IsAuroraEnable`))
    (return)
    (else
      (bind __isauroraenable (`self.TimeControl`))
      (set `self.IsAuroraEnable` __isauroraenable)
      (`self.VariablesControl` (`self.IsAuroraEnable`))
      (return))))

(fn `CalcRandomHour`
  (returns (_RandomHour :type Integer))
  (locals (RandomHourLoc :type Integer :default 0))
  (if (<= (`self.HourEnable`) (`self.HourDisable`))
    (return (`KismetMathLibrary.RandomIntegerInRange` (`self.HourEnable`) (`self.HourDisable`)))
    (else
      (set `local.RandomHourLoc` (`KismetMathLibrary.RandomIntegerInRange` (`self.HourEnable`) (+ (`self.HourDisable`) 23)))
      (if (> (`local.RandomHourLoc`) 23)
        (return (- (`local.RandomHourLoc`) 23))
        (else
          (return (`local.RandomHourLoc`)))))))

(fn `CheckCalendarLimits`
  (returns (IsPossible :type Boolean))
  (locals (MonthDisableLoc :type Integer) (DayDisableLoc :type Integer) (HourDisableLoc :type Integer))
  (if (> (`self.MonthEnable`) (`self.MonthDisable`))
    (set `local.MonthDisableLoc` (+ (`self.MonthDisable`) 12))
    (else
      (set `local.MonthDisableLoc` (`self.MonthDisable`))))
  (if (> (`self.DayEnable`) (`self.DayDisable`))
    (set `local.DayDisableLoc` (+ (`self.DayDisable`) 30))
    (else
      (set `local.DayDisableLoc` (`self.DayDisable`))))
  (if (> (`self.HourEnable`) (`self.HourDisable`))
    (set `local.HourDisableLoc` (+ (`self.HourDisable`) 23))
    (else
      (set `local.HourDisableLoc` (`self.HourDisable`))))
  (return (and (and (>= (`/Game/SkyConstruct/Blueprints/BP_SkyConstructMain.Months` (`self.BP_SkyConstructMain`)) (`self.MonthEnable`)) (<= (`/Game/SkyConstruct/Blueprints/BP_SkyConstructMain.Months` (`self.BP_SkyConstructMain`)) (`local.MonthDisableLoc`))) (and (>= (`/Game/SkyConstruct/Blueprints/BP_SkyConstructMain.Days` (`self.BP_SkyConstructMain`)) (`self.DayEnable`)) (<= (`/Game/SkyConstruct/Blueprints/BP_SkyConstructMain.Days` (`self.BP_SkyConstructMain`)) (`local.DayDisableLoc`))) (and (>= (`/Game/SkyConstruct/Blueprints/BP_SkyConstructMain.Hours` (`self.BP_SkyConstructMain`)) (`self.HourEnable`)) (<= (`/Game/SkyConstruct/Blueprints/BP_SkyConstructMain.Hours` (`self.BP_SkyConstructMain`)) (`local.HourDisableLoc`))))))

(fn `CheckDuration`
  (returns (IsPossible :type Boolean))
  (locals (TotalTimeLoc :type "Timespan Structure") (TotalMinutesLoc :type Integer :default 0))
  (set `local.TotalTimeLoc` (- (`KismetMathLibrary.Now`) (`self.TimeOfStart`)))
  (set `local.TotalMinutesLoc` (`KismetMathLibrary.FTrunc` (`KismetMathLibrary.GetTotalMinutes` (`local.TotalTimeLoc`))))
  (return (>= (`self.Duration`) (`local.TotalMinutesLoc`))))

(fn `CheckOnMaximum`
  (returns (IsMaximum :type Boolean))
  (locals (IsInterpA_Layer1_BaseScaleMax :type Boolean :default true) (IsInterpA_Layer2_BaseScaleMax :type Boolean :default true) (`IsInterpAurora PhaseMax` :type Boolean :default true) (`IsInterpAurora IntensityMax` :type Boolean :default true) (`IsInterpBlur AmountMax` :type Boolean :default true))
  (if (`self.IsInterpA_Layer1_BaseScale`)
    (set `local.IsInterpA_Layer1_BaseScaleMax` (>= (`self.A_Layer1_BaseScale`) (`self.A_Layer1_BaseScaleMax`))))
  (if (`self.IsInterpA_Layer2_BaseScale`)
    (set `local.IsInterpA_Layer2_BaseScaleMax` (>= (`self.A_Layer2_BaseScale`) (`self.A_Layer2_BaseScaleMax`))))
  (if (`self.IsInterpAurora Phase`)
    (set `local.IsInterpAurora PhaseMax` (>= (`self.Aurora Phase`) (`self.Aurora PhaseMax`))))
  (if (`self.IsInterpAurora Intensity`)
    (set `local.IsInterpAurora IntensityMax` (>= (`self.Aurora Intensity`) (`self.Aurora IntensityMax`))))
  (if (`self.IsInterpBlur Amount`)
    (set `local.IsInterpBlur AmountMax` (>= (`self.Blur Amount`) (`self.Blur AmountMax`))))
  (return (and (`local.IsInterpA_Layer1_BaseScaleMax`) (`local.IsInterpA_Layer2_BaseScaleMax`) (`local.IsInterpAurora PhaseMax`) (`local.IsInterpAurora IntensityMax`) (`local.IsInterpBlur AmountMax`))))

(fn `CheckOnMinimum`
  (returns (IsMinimum :type Boolean))
  (locals (IsInterpA_Layer1_BaseScaleMin :type Boolean :default true) (IsInterpA_Layer2_BaseScaleMin :type Boolean :default true) (`IsInterpAurora PhaseMin` :type Boolean :default true) (`IsInterpAurora IntensityMin` :type Boolean :default true) (`IsInterpBlur AmountMin` :type Boolean :default true))
  (if (`self.IsInterpA_Layer1_BaseScale`)
    (set `local.IsInterpA_Layer1_BaseScaleMin` (<= (`self.A_Layer1_BaseScale`) (`self.A_Layer1_BaseScaleMin`))))
  (if (`self.IsInterpA_Layer2_BaseScale`)
    (set `local.IsInterpA_Layer2_BaseScaleMin` (<= (`self.A_Layer2_BaseScale`) (`self.A_Layer2_BaseScaleMin`))))
  (if (`self.IsInterpAurora Phase`)
    (set `local.IsInterpAurora PhaseMin` (<= (`self.Aurora Phase`) (`self.Aurora PhaseMin`))))
  (if (`self.IsInterpAurora Intensity`)
    (set `local.IsInterpAurora IntensityMin` (<= (`self.Aurora Intensity`) (`self.Aurora IntensityMin`))))
  (if (`self.IsInterpBlur Amount`)
    (set `local.IsInterpBlur AmountMin` (<= (`self.Blur Amount`) (`self.Blur AmountMin`))))
  (return (and (`local.IsInterpA_Layer1_BaseScaleMin`) (`local.IsInterpA_Layer2_BaseScaleMin`) (`local.IsInterpAurora PhaseMin`) (`local.IsInterpAurora IntensityMin`) (`local.IsInterpBlur AmountMin`))))

(fn `CheckPause`
  (returns (IsPossible :type Boolean))
  (locals (TotalTimeLoc :type "Timespan Structure") (TotalMinutesLoc :type Integer :default 0))
  (set `local.TotalTimeLoc` (- (`KismetMathLibrary.Now`) (`self.TimeOfStop`)))
  (set `local.TotalMinutesLoc` (`KismetMathLibrary.FTrunc` (`KismetMathLibrary.GetTotalMinutes` (`local.TotalTimeLoc`))))
  (return (< (`self.PauseBetweenRuns`) (`local.TotalMinutesLoc`))))

(fn `InterpolateVariables`
  (if (`self.IsInterpA_Layer1_BaseScale`)
    (set `self.A_Layer1_BaseScale` (`KismetMathLibrary.FInterpTo_Constant` (`self.A_Layer1_BaseScale`) (`self.A_Layer1_BaseScaleMax`) (`self.InterpolateVariablesDeltaTime`) (`self.InterpolateSpeedA_Layer1_BaseScale`))))
  (if (`self.IsInterpA_Layer2_BaseScale`)
    (set `self.A_Layer2_BaseScale` (`KismetMathLibrary.FInterpTo_Constant` (`self.A_Layer2_BaseScale`) (`self.A_Layer2_BaseScaleMax`) (`self.InterpolateVariablesDeltaTime`) (`self.InterpolateSpeedA_Layer2_BaseScale`))))
  (if (`self.IsInterpAurora Intensity`)
    (set `self.Aurora Intensity` (`KismetMathLibrary.FInterpTo_Constant` (`self.Aurora Intensity`) (`self.Aurora IntensityMax`) (`self.InterpolateVariablesDeltaTime`) (`self.InterpolateSpeedAurora Intensity`))))
  (if (`self.IsInterpAurora Phase`)
    (set `self.Aurora Phase` (`KismetMathLibrary.FInterpTo_Constant` (`self.Aurora Phase`) (`self.Aurora PhaseMax`) (`self.InterpolateVariablesDeltaTime`) (`self.InterpolateSpeedAurora Phase`))))
  (if (`self.IsInterpBlur Amount`)
    (set `self.Blur Amount` (`KismetMathLibrary.FInterpTo_Constant` (`self.Blur Amount`) (`self.Blur AmountMax`) (`self.InterpolateVariablesDeltaTime`) (`self.InterpolateSpeedBlur Amount`))))
  (`self.SetMaterialParameters`)
  (if (`self.CheckOnMaximum`)
    (`self.StopInterpolateVariables`)
    (bind _returnvalue (`KismetSystemLibrary.K2_SetTimer` null "ReverseInterpolateVariables" (`self.InterpolateVariablesDeltaTime`) true))
    (set `self.InterpolateVariablesTimer` _returnvalue)
    (return)
    (else
      (return))))

(fn `ReverseInterpolateVariables`
  (if (`self.IsInterpA_Layer1_BaseScale`)
    (set `self.A_Layer1_BaseScale` (`KismetMathLibrary.FInterpTo_Constant` (`self.A_Layer1_BaseScale`) (`self.A_Layer1_BaseScaleMin`) (`self.InterpolateVariablesDeltaTime`) (`self.InterpolateSpeedA_Layer1_BaseScale`))))
  (if (`self.IsInterpA_Layer2_BaseScale`)
    (set `self.A_Layer2_BaseScale` (`KismetMathLibrary.FInterpTo_Constant` (`self.A_Layer2_BaseScale`) (`self.A_Layer2_BaseScaleMin`) (`self.InterpolateVariablesDeltaTime`) (`self.InterpolateSpeedA_Layer2_BaseScale`))))
  (if (`self.IsInterpAurora Intensity`)
    (set `self.Aurora Intensity` (`KismetMathLibrary.FInterpTo_Constant` (`self.Aurora Intensity`) (`self.Aurora IntensityMin`) (`self.InterpolateVariablesDeltaTime`) (`self.InterpolateSpeedAurora Intensity`))))
  (if (`self.IsInterpAurora Phase`)
    (set `self.Aurora Phase` (`KismetMathLibrary.FInterpTo_Constant` (`self.Aurora Phase`) (`self.Aurora PhaseMin`) (`self.InterpolateVariablesDeltaTime`) (`self.InterpolateSpeedAurora Phase`))))
  (if (`self.IsInterpBlur Amount`)
    (set `self.Blur Amount` (`KismetMathLibrary.FInterpTo_Constant` (`self.Blur Amount`) (`self.Blur AmountMin`) (`self.InterpolateVariablesDeltaTime`) (`self.InterpolateSpeedBlur Amount`))))
  (`self.SetMaterialParameters`)
  (if (`self.CheckOnMinimum`)
    (`self.StopInterpolateVariables`)
    (bind _returnvalue (`KismetSystemLibrary.K2_SetTimer` null "InterpolateVariables" (`self.InterpolateVariablesDeltaTime`) true))
    (set `self.InterpolateVariablesTimer` _returnvalue)
    (return)
    (else
      (return))))

(fn `SetDuration`
  (set `self.Duration` (`KismetMathLibrary.RandomIntegerInRange` (`self.DurationMin`) (`self.DurationMax`)))
  (return))

(fn `SetIsInterpBooleanVariables`
  (set `self.IsInterpA_Layer1_BaseScale` (`KismetMathLibrary.RandomBool`))
  (set `self.IsInterpA_Layer2_BaseScale` (`KismetMathLibrary.RandomBool`))
  (set `self.IsInterpAurora Phase` (`KismetMathLibrary.RandomBool`))
  (set `self.IsInterpAurora Intensity` (`KismetMathLibrary.RandomBool`))
  (set `self.IsInterpBlur Amount` (`KismetMathLibrary.RandomBool`))
  (return))

(fn `SetMaterialParameters`
  (`KismetMaterialLibrary.SetScalarParameterValue` "/Game/SkyConstruct/Materials/MaterialParameterCollections/MPC_Aurora.MPC_Aurora" "A_Layer1_BaseScale" (`self.A_Layer1_BaseScale`))
  (`KismetMaterialLibrary.SetScalarParameterValue` "/Game/SkyConstruct/Materials/MaterialParameterCollections/MPC_Aurora.MPC_Aurora" "A_Layer2_BaseScale" (`self.A_Layer2_BaseScale`))
  (`KismetMaterialLibrary.SetScalarParameterValue` "/Game/SkyConstruct/Materials/MaterialParameterCollections/MPC_Aurora.MPC_Aurora" "Aurora Intensity" (`self.Aurora Intensity`))
  (`KismetMaterialLibrary.SetScalarParameterValue` "/Game/SkyConstruct/Materials/MaterialParameterCollections/MPC_Aurora.MPC_Aurora" "Aurora Phase" (`self.Aurora Phase`))
  (`KismetMaterialLibrary.SetScalarParameterValue` "/Game/SkyConstruct/Materials/MaterialParameterCollections/MPC_Aurora.MPC_Aurora" "Aurora Speed" (`self.Aurora Speed`))
  (`KismetMaterialLibrary.SetScalarParameterValue` "/Game/SkyConstruct/Materials/MaterialParameterCollections/MPC_Aurora.MPC_Aurora" "Blur Amount" (`self.Blur Amount`))
  (return))

(fn `SetRandomVariables`
  (set `self.A_Layer1_BaseScale` (`KismetMathLibrary.RandomFloatInRange` (`self.A_Layer1_BaseScaleMin`) (`self.A_Layer1_BaseScaleMax`)))
  (set `self.A_Layer2_BaseScale` (`KismetMathLibrary.RandomFloatInRange` (`self.A_Layer2_BaseScaleMin`) (`self.A_Layer2_BaseScaleMax`)))
  (set `self.Aurora Intensity` (`KismetMathLibrary.RandomFloatInRange` (`self.Aurora IntensityMin`) (`self.Aurora IntensityMax`)))
  (set `self.Aurora Phase` (`KismetMathLibrary.RandomFloatInRange` (`self.Aurora PhaseMin`) (`self.Aurora PhaseMax`)))
  (set `self.Aurora Speed` (`KismetMathLibrary.RandomFloatInRange` (`self.Aurora SpeedMin`) (`self.Aurora SpeedMax`)))
  (set `self.Blur Amount` (`KismetMathLibrary.RandomFloatInRange` (`self.Blur AmountMin`) (`self.Blur AmountMax`)))
  (return))

(fn `StartInterpolateVariables`
  (`self.SetIsInterpBooleanVariables`)
  (`self.SetRandomVariables`)
  (`self.SetMaterialParameters`)
  (`self.SetDuration`)
  (set `self.TimeOfStart` (`KismetMathLibrary.Now`))
  (bind _returnvalue (`KismetSystemLibrary.K2_SetTimer` null "InterpolateVariables" (`self.InterpolateVariablesDeltaTime`) true))
  (set `self.InterpolateVariablesTimer` _returnvalue)
  (return))

(fn `StopInterpolateVariables`
  (`KismetSystemLibrary.K2_ClearAndInvalidateTimerHandle` (`self.InterpolateVariablesTimer`))
  (return))

(fn `TimeControl`
  (returns (_IsAuroraEnable :type Boolean))
  (locals (IsAuroraShouldEnableLoc :type Boolean :default true))
  (if (`self.IsAuroraEnable`)
    ;[0.5 1 0] Если включена, то проверять продолжительность работы.
    (return (`self.CheckDuration`))
    (else
      ;[1 0.6328 0] Если выключена, то проверять на интервал времени, в который может работать.
      (if (`self.CheckCalendarLimits`)
        ;[1 0 0.3047] Если в рабочем интервале, то проверить, была ли ранее запущена в этом интервале.
        (if (`self.IsStartInCurrentInterval`)
          (return false)
          (else
            ;[1 0.04688 0] Если была ранее запущена, то проверить, был ли расчет времени запуска.
            (if (`self.IsRandomHourCalculated`)
              ;[1 0.4453 0] Если время запуска было расчитано, то проверить, пришло ли время.
              (if (== (`/Game/SkyConstruct/Blueprints/BP_SkyConstructMain.Hours` (`self.BP_SkyConstructMain`)) (`self.RandomHourOfStart`))
                ;[0.9219 1 0] Если время пришло - запустить.
                (set `self.IsStartInCurrentInterval` true)
                (return (`KismetMathLibrary.RandomBoolWithWeight` (`self.WeightOfRandomRun`)))
                (else
                  (return false)))
              (else
                ;[0 0.5078 1] Расчитать время запуска и уйти на следующую итерацию таймера.
                (set `self.RandomHourOfStart` (`self.CalcRandomHour`))
                (set `self.IsRandomHourCalculated` true)
                (return false)))))
        (else
          ;[0.3594 0 1] Если не в рабочем интервале, то подготавливать к следующему интервалу.
          (set `self.IsStartInCurrentInterval` false)
          (set `self.IsRandomHourCalculated` false)
          (return false))))))

(fn `VariablesControl`
  (params (_IsAuroraEnable :type Boolean))
  (locals (IsAuroraEnableLoc :type Boolean) (IsAuroraWasEnabledLoc :type Boolean :default false))
  (set `local.IsAuroraEnableLoc` _IsAuroraEnable)
  ;[1 0 0.2812] Позволяет вручную менять параметры во время работы. Подходит для тестирования.
  (if (`local.IsAuroraEnableLoc`)
    (if (`|EnumEquality` (`self.EAuroraVariablesControlType`) "NewEnumerator0")
      (`self.StopInterpolateVariables`)
      (`self.SetMaterialParameters`)))
  ;[0.4766 0 1] Изменить состояние включено/выключено только если входные данные по включению изменились.
  (bind _returnvalue (`KismetMaterialLibrary.GetScalarParameterValue` "/Game/SkyConstruct/Materials/MaterialParameterCollections/MPC_Aurora.MPC_Aurora" "IsAuroraEnabled"))
  (set `local.IsAuroraWasEnabledLoc` (`KismetMathLibrary.Conv_IntToBool` (`KismetMathLibrary.FTrunc` _returnvalue)))
  (if (== (`local.IsAuroraWasEnabledLoc`) (`local.IsAuroraEnableLoc`))
    (return)
    (else
      (`KismetMaterialLibrary.SetScalarParameterValue` "/Game/SkyConstruct/Materials/MaterialParameterCollections/MPC_Aurora.MPC_Aurora" "IsAuroraEnabled" (`KismetMathLibrary.Conv_BoolToDouble` (`local.IsAuroraEnableLoc`)))
      (`self.StopInterpolateVariables`)
      (if (`local.IsAuroraEnableLoc`)
        (switch `/Game/SkyConstruct/Blueprints/Enums/EAuroraVariablesControlType` (`self.EAuroraVariablesControlType`)
          (:`NewEnumerator0`
            (return))
          (:`NewEnumerator2`
            (`self.StartInterpolateVariables`)
            (return)))
        (else
          (return))))))