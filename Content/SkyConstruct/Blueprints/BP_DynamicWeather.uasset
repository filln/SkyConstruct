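; Weather component for BP_SkyConstructMain that randomly changes the sky's weather over time, weighted by month.
; DynamicWeatherSystem runs a TimeSpeed-scaled timer that periodically rolls one of five weather types from monthly tables, plus random fog and wind.
; Between rolls, DifferentWeather interpolates the owner's sun, moon, sky, cloud and fog values toward that preset.
; Rain and snow attach to the player camera, appearing only once cloud coverage exceeds 0.5.
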(event `self.ReceiveBeginPlay`
  (bind _asbp_sky_construct_main (cast `/Game/SkyConstruct/Blueprints/BP_SkyConstructMain` (`self.GetOwner`))
    (:`then`
      (set `self.BP_SkyConstructMain` _asbp_sky_construct_main))
    (:`CastFailed`
      (`KismetSystemLibrary.PrintString` "BP_SkyConstructMain CastFailed"))))

(fn `ActivateRain`
  (params (DeltaTime_ :type "Float (double-precision)"))
  (set `/Game/SkyConstruct/Blueprints/BP_SkyConstructMain.PPRainIntensity` (`KismetMathLibrary.FInterpTo` (`/Game/SkyConstruct/Blueprints/BP_SkyConstructMain.PPRainIntensity` (`self.BP_SkyConstructMain`)) 1.0 DeltaTime_ (`/Game/SkyConstruct/Blueprints/BP_SkyConstructMain.WeatherTransitionSpeed` (`self.BP_SkyConstructMain`))) (`self.BP_SkyConstructMain`))
  (if (> (`/Game/SkyConstruct/Blueprints/BP_SkyConstructMain.Coverage` (`self.BP_SkyConstructMain`)) 0.5)
    (`SceneComponent.SetVisibility` (`/Game/SkyConstruct/Blueprints/BP_SkyConstructMain.Rain` (`self.BP_SkyConstructMain`)) true false)
    (return)
    (else
      (return))))

(fn `ActivateSnow`
  (if (> (`/Game/SkyConstruct/Blueprints/BP_SkyConstructMain.Coverage` (`self.BP_SkyConstructMain`)) 0.5)
    (`SceneComponent.SetVisibility` (`/Game/SkyConstruct/Blueprints/BP_SkyConstructMain.Snow` (`self.BP_SkyConstructMain`)) true false)
    (return)
    (else
      (return))))

(fn `CloudyFoggyWeather`
  (params (DeltaTime_ :type "Float (double-precision)"))
  (bind (_cloudyfoggyweather_sunintensity _cloudyfoggyweather_sunbloomstrength _cloudyfoggyweather_bloomscale _cloudyfoggyweather_moonintensity _cloudyfoggyweather_moonbloomstrength _cloudyfoggyweather_moonbloomscale _cloudyfoggyweather_skybrightness _cloudyfoggyweather_starsbrightness _cloudyfoggyweather_skylightintensity _cloudyfoggyweather_skylightcolor _cloudyfoggyweather_coverage _cloudyfoggyweather_density _cloudyfoggyweather_lightintensity _cloudyfoggyweather_shadowsize _cloudyfoggyweather_ambientintensity _cloudyfoggyweather_exfogdensity _cloudyfoggyweather_foginscolor) (break `/Game/DynamicVolumetricSky/Blueprints/WeatherStructures/CloudyFoggyWeatherStructure` (`/Game/SkyConstruct/Blueprints/BP_SkyConstructMain.CloudyFoggyWeather` (`self.BP_SkyConstructMain`))))
  (`self.DifferentWeather` DeltaTime_ (make `/Game/SkyConstruct/Blueprints/WeatherStructures/DifferentWeatherTempStructure` _cloudyfoggyweather_sunintensity _cloudyfoggyweather_sunbloomstrength _cloudyfoggyweather_bloomscale _cloudyfoggyweather_moonintensity _cloudyfoggyweather_moonbloomstrength _cloudyfoggyweather_moonbloomscale _cloudyfoggyweather_skybrightness _cloudyfoggyweather_starsbrightness _cloudyfoggyweather_skylightintensity _cloudyfoggyweather_skylightcolor _cloudyfoggyweather_coverage _cloudyfoggyweather_density _cloudyfoggyweather_lightintensity _cloudyfoggyweather_shadowsize _cloudyfoggyweather_ambientintensity _cloudyfoggyweather_exfogdensity _cloudyfoggyweather_foginscolor))
  (`self.DeactivateRain` DeltaTime_)
  (`self.DeactivateSnow`))

(fn `CloudyWeather`
  (params (DeltaTime_ :type "Float (double-precision)"))
  (bind (_cloudyweather_sunintensity _cloudyweather_sunbloomstrength _cloudyweather_bloomscale _cloudyweather_moonintensity _cloudyweather_moonbloomstrength _cloudyweather_moonbloomscale _cloudyweather_skybrightness _cloudyweather_starsbrightness _cloudyweather_skylightintensity _cloudyweather_skylightcolor _cloudyweather_coverage _cloudyweather_lightintensity _cloudyweather_shadowsize _cloudyweather_ambientintensity _cloudyweather_exfogdensity _cloudyweather_foginscolor) (break `/Game/DynamicVolumetricSky/Blueprints/WeatherStructures/CloudyWeatherStructure` (`/Game/SkyConstruct/Blueprints/BP_SkyConstructMain.CloudyWeather` (`self.BP_SkyConstructMain`))))
  (`self.DifferentWeather` DeltaTime_ (make `/Game/SkyConstruct/Blueprints/WeatherStructures/DifferentWeatherTempStructure` _cloudyweather_sunintensity _cloudyweather_sunbloomstrength _cloudyweather_bloomscale _cloudyweather_moonintensity _cloudyweather_moonbloomstrength _cloudyweather_moonbloomscale _cloudyweather_skybrightness _cloudyweather_starsbrightness _cloudyweather_skylightintensity _cloudyweather_skylightcolor _cloudyweather_coverage 0.0 _cloudyweather_lightintensity _cloudyweather_shadowsize _cloudyweather_ambientintensity _cloudyweather_exfogdensity _cloudyweather_foginscolor))
  (`self.DeactivateRain` DeltaTime_)
  (`self.DeactivateSnow`))

(fn `DeactivateRain`
  (params (DeltaTime_ :type "Float (double-precision)"))
  (set `/Game/SkyConstruct/Blueprints/BP_SkyConstructMain.PPRainIntensity` (`KismetMathLibrary.FInterpTo` (`/Game/SkyConstruct/Blueprints/BP_SkyConstructMain.PPRainIntensity` (`self.BP_SkyConstructMain`)) 0.0 DeltaTime_ (`/Game/SkyConstruct/Blueprints/BP_SkyConstructMain.WeatherTransitionSpeed` (`self.BP_SkyConstructMain`))) (`self.BP_SkyConstructMain`))
  (`SceneComponent.SetVisibility` (`/Game/SkyConstruct/Blueprints/BP_SkyConstructMain.Rain` (`self.BP_SkyConstructMain`)) false false))

(fn `DeactivateSnow`
  (`SceneComponent.SetVisibility` (`/Game/SkyConstruct/Blueprints/BP_SkyConstructMain.Snow` (`self.BP_SkyConstructMain`)) false false))

(fn `DifferentWeather`
  (params (DeltaTime_ :type "Float (double-precision)") (DifferentWeatherTempStructure_ :type "/Game/SkyConstruct/Blueprints/WeatherStructures/DifferentWeatherTempStructure Structure"))
  (locals (WeatherTransitionSpeedLoc :type "Float (double-precision)" :default 0.0) (DeltaTimeLoc :type "Float (double-precision)") (SunIntensityLoc :type "Float (double-precision)") (SunBloomStrengthLoc :type "Float (double-precision)") (BloomScaleLoc :type "Float (double-precision)") (MoonIntensityLoc :type "Float (double-precision)") (MoonBloomStrengthLoc :type "Float (double-precision)") (MoonBloomScaleLoc :type "Float (double-precision)") (SkyBrightnessLoc :type "Float (double-precision)") (StarsBrightnessLoc :type "Float (double-precision)") (SkyLightIntensityLoc :type "Float (double-precision)") (SkyLightColorLoc :type "LinearColor Structure") (CoverageLoc :type "Float (double-precision)") (DensityLoc :type "Float (double-precision)") (LightIntensityLoc :type "Float (double-precision)") (ShadowSizeLoc :type "Float (double-precision)") (AmbientIntensityLoc :type "Float (double-precision)") (ExFogDensityLoc :type "Float (double-precision)") (FogInsColorLoc :type "LinearColor Structure"))
  (set `local.WeatherTransitionSpeedLoc` (`/Game/SkyConstruct/Blueprints/BP_SkyConstructMain.WeatherTransitionSpeed` (`self.BP_SkyConstructMain`)))
  (set `local.DeltaTimeLoc` DeltaTime_)
  (set `local.SunIntensityLoc` DifferentWeatherTempStructure__SunIntensity_7_793AB47741294F27C2FFB88D049C9993)
  (set `local.SunBloomStrengthLoc` DifferentWeatherTempStructure__SunBloomStrength_11_0611020E4A34886EBCE790AFE359E2CE)
  (set `local.BloomScaleLoc` DifferentWeatherTempStructure__BloomScale_14_E44695854A4E26D8C69DEF8F2559E340)
  (set `local.MoonIntensityLoc` DifferentWeatherTempStructure__MoonIntensity_19_DAFCD06846693276389DB99813A160D7)
  (set `local.MoonBloomStrengthLoc` DifferentWeatherTempStructure__MoonBloomStrength_22_310A34B943D97FB1CE1CC8A6E1617E5E)
  (set `local.MoonBloomScaleLoc` DifferentWeatherTempStructure__MoonBloomScale_23_9D71A7004A428B0C4CFA85BDF3FB76F7)
  (set `local.SkyBrightnessLoc` DifferentWeatherTempStructure__SkyBrightness_26_3E78343B46C86625E5CDD38EEFC466E3)
  (set `local.StarsBrightnessLoc` DifferentWeatherTempStructure__StarsBrightness_28_0752478D4A12384B8EADEBA4C3F21B73)
  (set `local.SkyLightIntensityLoc` DifferentWeatherTempStructure__SkyLightIntensity_30_AA11A2064794BFF7F68961A027AE0F83)
  (set `local.SkyLightColorLoc` DifferentWeatherTempStructure__SkyLightColor_34_C28F018945B48850D7C675A857D89D35)
  (set `local.CoverageLoc` DifferentWeatherTempStructure__Coverage_37_B60860654F679AFD6568DBB4E7AF4C43)
  (set `local.DensityLoc` DifferentWeatherTempStructure__Density_39_FB4B9EFB4880190275498CB8924A1486)
  (set `local.LightIntensityLoc` DifferentWeatherTempStructure__LightIntensity_53_B3E2B7D84C38FBC847C518B85EE9A3D2)
  (set `local.ShadowSizeLoc` DifferentWeatherTempStructure__ShadowSize_67_0AC7B06E4B6BA0666A58719B2C3E5516)
  (set `local.AmbientIntensityLoc` DifferentWeatherTempStructure__AmbientIntensity_64_8BA974154172A8D69134F2B716C17A24)
  (set `local.ExFogDensityLoc` DifferentWeatherTempStructure__ExFogDensity_45_45E8A2D0420787FE4408CE82AA4F18F1)
  (set `local.FogInsColorLoc` DifferentWeatherTempStructure__FogInsColor_61_67CE440F436F56BED23C0194932C1C4B)
  (`|ExecutionSequence`
    (:`then_0`
      ;[0.4219 0.4037 0.3362] CloudyFoggyWeather
      (set `/Game/SkyConstruct/Blueprints/BP_SkyConstructMain.SunIntensityTarget` (`KismetMathLibrary.FInterpTo` (`/Game/SkyConstruct/Blueprints/BP_SkyConstructMain.SunIntensityTarget` (`self.BP_SkyConstructMain`)) (`local.SunIntensityLoc`) (`local.DeltaTimeLoc`) (`local.WeatherTransitionSpeedLoc`)) (`self.BP_SkyConstructMain`))
      (set `/Game/SkyConstruct/Blueprints/BP_SkyConstructMain.SunBloomStrength` (`KismetMathLibrary.FInterpTo` (`/Game/SkyConstruct/Blueprints/BP_SkyConstructMain.SunBloomStrength` (`self.BP_SkyConstructMain`)) (`local.SunBloomStrengthLoc`) (`local.DeltaTimeLoc`) (`local.WeatherTransitionSpeedLoc`)) (`self.BP_SkyConstructMain`))
      (set `/Game/SkyConstruct/Blueprints/BP_SkyConstructMain.BloomScale` (`KismetMathLibrary.FInterpTo` (`/Game/SkyConstruct/Blueprints/BP_SkyConstructMain.BloomScale` (`self.BP_SkyConstructMain`)) (`local.BloomScaleLoc`) (`local.DeltaTimeLoc`) (`local.WeatherTransitionSpeedLoc`)) (`self.BP_SkyConstructMain`))
      (set `/Game/SkyConstruct/Blueprints/BP_SkyConstructMain.MoonIntensityTarget` (`KismetMathLibrary.FInterpTo` (`/Game/SkyConstruct/Blueprints/BP_SkyConstructMain.MoonIntensityTarget` (`self.BP_SkyConstructMain`)) (`local.MoonIntensityLoc`) (`local.DeltaTimeLoc`) (`local.WeatherTransitionSpeedLoc`)) (`self.BP_SkyConstructMain`))
      (set `/Game/SkyConstruct/Blueprints/BP_SkyConstructMain.MoonBloomStrength` (`KismetMathLibrary.FInterpTo` (`/Game/SkyConstruct/Blueprints/BP_SkyConstructMain.MoonBloomStrength` (`self.BP_SkyConstructMain`)) (`local.MoonBloomStrengthLoc`) (`local.DeltaTimeLoc`) (`local.WeatherTransitionSpeedLoc`)) (`self.BP_SkyConstructMain`))
      (set `/Game/SkyConstruct/Blueprints/BP_SkyConstructMain.MoonBloomScale` (`KismetMathLibrary.FInterpTo` (`/Game/SkyConstruct/Blueprints/BP_SkyConstructMain.MoonBloomScale` (`self.BP_SkyConstructMain`)) (`local.MoonBloomScaleLoc`) (`local.DeltaTimeLoc`) (`local.WeatherTransitionSpeedLoc`)) (`self.BP_SkyConstructMain`)))
    (:`then_1`
      (set `/Game/SkyConstruct/Blueprints/BP_SkyConstructMain.SkyBrightness` (`KismetMathLibrary.FInterpTo` (`/Game/SkyConstruct/Blueprints/BP_SkyConstructMain.SkyBrightness` (`self.BP_SkyConstructMain`)) (`local.SkyBrightnessLoc`) (`local.DeltaTimeLoc`) (`local.WeatherTransitionSpeedLoc`)) (`self.BP_SkyConstructMain`))
      (set `/Game/SkyConstruct/Blueprints/BP_SkyConstructMain.StarsBrightness` (`KismetMathLibrary.FInterpTo` (`/Game/SkyConstruct/Blueprints/BP_SkyConstructMain.StarsBrightness` (`self.BP_SkyConstructMain`)) (`local.StarsBrightnessLoc`) (`local.DeltaTimeLoc`) (`local.WeatherTransitionSpeedLoc`)) (`self.BP_SkyConstructMain`))
      (set `/Game/SkyConstruct/Blueprints/BP_SkyConstructMain.SkyLightIntensity` (`KismetMathLibrary.FInterpTo` (`/Game/SkyConstruct/Blueprints/BP_SkyConstructMain.SkyLightIntensity` (`self.BP_SkyConstructMain`)) (`local.SkyLightIntensityLoc`) (`local.DeltaTimeLoc`) (`local.WeatherTransitionSpeedLoc`)) (`self.BP_SkyConstructMain`))
      (set `/Game/SkyConstruct/Blueprints/BP_SkyConstructMain.SkyLightColor` (`KismetMathLibrary.CInterpTo` (`/Game/SkyConstruct/Blueprints/BP_SkyConstructMain.SkyLightColor` (`self.BP_SkyConstructMain`)) (`local.SkyLightColorLoc`) (`local.DeltaTimeLoc`) (`local.WeatherTransitionSpeedLoc`)) (`self.BP_SkyConstructMain`))
      (set `/Game/SkyConstruct/Blueprints/BP_SkyConstructMain.Coverage` (`KismetMathLibrary.FInterpTo` (`/Game/SkyConstruct/Blueprints/BP_SkyConstructMain.Coverage` (`self.BP_SkyConstructMain`)) (`local.CoverageLoc`) (`local.DeltaTimeLoc`) (`local.WeatherTransitionSpeedLoc`)) (`self.BP_SkyConstructMain`))
      (set `/Game/SkyConstruct/Blueprints/BP_SkyConstructMain.LightIntensity` (`KismetMathLibrary.FInterpTo` (`/Game/SkyConstruct/Blueprints/BP_SkyConstructMain.LightIntensity` (`self.BP_SkyConstructMain`)) (`local.LightIntensityLoc`) (`local.DeltaTimeLoc`) (`local.WeatherTransitionSpeedLoc`)) (`self.BP_SkyConstructMain`))
      (set `/Game/SkyConstruct/Blueprints/BP_SkyConstructMain.ShadowSize` (`KismetMathLibrary.FInterpTo` (`/Game/SkyConstruct/Blueprints/BP_SkyConstructMain.ShadowSize` (`self.BP_SkyConstructMain`)) (`local.ShadowSizeLoc`) (`local.DeltaTimeLoc`) (`local.WeatherTransitionSpeedLoc`)) (`self.BP_SkyConstructMain`)))
    (:`then_2`
      (set `/Game/SkyConstruct/Blueprints/BP_SkyConstructMain.AmbientIntensity` (`KismetMathLibrary.FInterpTo` (`/Game/SkyConstruct/Blueprints/BP_SkyConstructMain.AmbientIntensity` (`self.BP_SkyConstructMain`)) (`local.AmbientIntensityLoc`) (`local.DeltaTimeLoc`) (`local.WeatherTransitionSpeedLoc`)) (`self.BP_SkyConstructMain`))
      (set `/Game/SkyConstruct/Blueprints/BP_SkyConstructMain.ExFogDensity` (`KismetMathLibrary.FInterpTo` (`/Game/SkyConstruct/Blueprints/BP_SkyConstructMain.ExFogDensity` (`self.BP_SkyConstructMain`)) (`local.ExFogDensityLoc`) (`local.DeltaTimeLoc`) (`local.WeatherTransitionSpeedLoc`)) (`self.BP_SkyConstructMain`))
      (set `/Game/SkyConstruct/Blueprints/BP_SkyConstructMain.FogInsColor` (`KismetMathLibrary.CInterpTo` (`/Game/SkyConstruct/Blueprints/BP_SkyConstructMain.FogInsColor` (`self.BP_SkyConstructMain`)) (`local.FogInsColorLoc`) (`local.DeltaTimeLoc`) (`local.WeatherTransitionSpeedLoc`)) (`self.BP_SkyConstructMain`))
      (set `/Game/SkyConstruct/Blueprints/BP_SkyConstructMain.CloudWind` (`KismetMathLibrary.CInterpTo` (`/Game/SkyConstruct/Blueprints/BP_SkyConstructMain.CloudWind` (`self.BP_SkyConstructMain`)) (`/Game/SkyConstruct/Blueprints/BP_SkyConstructMain.CloudWindTarget` (`self.BP_SkyConstructMain`)) (`local.DeltaTimeLoc`) (/ (`local.WeatherTransitionSpeedLoc`) 10.0)) (`self.BP_SkyConstructMain`)))))

(fn `DynamicWeatherSystem`
  (params (DeltaTime_ :type "Float (double-precision)"))
  (locals (DeltaTimeLoc :type "Float (double-precision)"))
  (bind _deltatimeloc (`local.DeltaTimeLoc`))
  (bind _deltatimeloc_2 (`local.DeltaTimeLoc`))
  ;[0.01 0.01 0.01] Infinite Loop
  (if (`/Game/SkyConstruct/Blueprints/BP_SkyConstructMain.DynamicWeatherSystem?` (`self.BP_SkyConstructMain`))
    (set `local.DeltaTimeLoc` DeltaTime_)
    (`/Engine/EditorBlueprintResources/StandardMacros.Do N` 999999999 :!label _label
      (:`Exit`
        (set `/Game/SkyConstruct/Blueprints/BP_SkyConstructMain.WeatherLoop1` (+ (`/Game/SkyConstruct/Blueprints/BP_SkyConstructMain.WeatherLoop1` (`self.BP_SkyConstructMain`)) (* (`KismetMathLibrary.Conv_IntToDouble` (`/Game/SkyConstruct/Blueprints/BP_SkyConstructMain.TimeSpeed` (`self.BP_SkyConstructMain`))) (`local.DeltaTimeLoc`))) (`self.BP_SkyConstructMain`))
        (set `/Game/SkyConstruct/Blueprints/BP_SkyConstructMain.WeatherLoop2` (`KismetMathLibrary.MapRangeClamped` (`/Game/SkyConstruct/Blueprints/BP_SkyConstructMain.WeatherLoop1` (`self.BP_SkyConstructMain`)) 0.0 (* (* (/ 1.0 (`/Game/SkyConstruct/Blueprints/BP_SkyConstructMain.WeatherFrequency` (`self.BP_SkyConstructMain`))) 60.0) (`KismetMathLibrary.Conv_IntToDouble` (`/Game/SkyConstruct/Blueprints/BP_SkyConstructMain.TimeSpeed` (`self.BP_SkyConstructMain`)))) 0.0 1.0) (`self.BP_SkyConstructMain`))
        (if (== (`/Game/SkyConstruct/Blueprints/BP_SkyConstructMain.WeatherLoop2` (`self.BP_SkyConstructMain`)) 1.0)
          ;[0.1164 0.1576 0.3854] Weather Generation
          (set `self.WeatherChance` (`self.MonthlyWeatherChance`))
          (bind _output_get (set `/Game/SkyConstruct/Blueprints/BP_SkyConstructMain.FoggyChance` (`KismetMathLibrary.RandomIntegerInRange` 0 1) (`self.BP_SkyConstructMain`)))
          (if (== _output_get 1)
            (set `/Game/SkyConstruct/Blueprints/BP_SkyConstructMain.Foggy?` true (`self.BP_SkyConstructMain`))
            (`self.SetWindProperties` 0.001 0.02)
            (else
              (set `/Game/SkyConstruct/Blueprints/BP_SkyConstructMain.Foggy?` false (`self.BP_SkyConstructMain`))
              (set `/Game/SkyConstruct/Blueprints/BP_SkyConstructMain.WindyChange` (`KismetMathLibrary.RandomIntegerInRange` 0 1) (`self.BP_SkyConstructMain`))
              (if (== (`/Game/SkyConstruct/Blueprints/BP_SkyConstructMain.WindyChange` (`self.BP_SkyConstructMain`)) 0)
                (set `/Game/SkyConstruct/Blueprints/BP_SkyConstructMain.Windy?` false (`self.BP_SkyConstructMain`))
                (`self.SetWindProperties` 0.001 0.008)
                (else
                  (set `/Game/SkyConstruct/Blueprints/BP_SkyConstructMain.Windy?` true (`self.BP_SkyConstructMain`))
                  (`self.SetWindProperties` 0.008 0.01)))))
          (set `/Game/SkyConstruct/Blueprints/BP_SkyConstructMain.WeatherLoop1` 0.0 (`self.BP_SkyConstructMain`))
          (goto _label :!via `Reset`)
          (else
            ;[1 0 0] Condition Check
            (if (`/Game/SkyConstruct/Blueprints/BP_SkyConstructMain.Foggy?` (`self.BP_SkyConstructMain`))
              (switch `int` (`self.WeatherChance`)
                (:`0`
                  ;[1 0 0.6797] Туманная погода.
                  (`self.SunnyFoggyWeather` _deltatimeloc_2))
                (:`1`
                  (`self.PartlyCloudyFoggyWeather` _deltatimeloc_2))
                (:`2`
                  (`self.CloudyFoggyWeather` _deltatimeloc_2))
                (:`3`
                  (`self.RainyFoggyWeather` _deltatimeloc_2))
                (:`4`
                  (`self.SnowyFoggyWeather` _deltatimeloc_2)))
              (else
                (switch `int` (`self.WeatherChance`)
                  (:`0`
                    ;[0 1 0.6719] Не туманная погода.
                    (`self.SunnyWeather` _deltatimeloc))
                  (:`1`
                    (`self.PartlyCloudyWeather` _deltatimeloc))
                  (:`2`
                    (`self.CloudyWeather` _deltatimeloc))
                  (:`3`
                    (`self.RainyWeather` _deltatimeloc))
                  (:`4`
                    (`self.SnowyWeather` _deltatimeloc)))))))))))

(fn `InitialiseWeather`
  (`|ExecutionSequence`
    (:`then_0`
      (set `self.WeatherChance` (`self.MonthlyWeatherChance`)))
    (:`then_1`
      (`SceneComponent.K2_AttachToComponent` (`/Game/SkyConstruct/Blueprints/BP_SkyConstructMain.Rain` (`self.BP_SkyConstructMain`)) (`PlayerCameraManager.TransformComponent` (`GameplayStatics.GetPlayerCameraManager` 0)) "None" "KeepRelative" "KeepRelative" "KeepRelative" true)
      (`SceneComponent.K2_AttachToComponent` (`/Game/SkyConstruct/Blueprints/BP_SkyConstructMain.Snow` (`self.BP_SkyConstructMain`)) (`PlayerCameraManager.TransformComponent` (`GameplayStatics.GetPlayerCameraManager` 0)) "None" "KeepRelative" "KeepRelative" "KeepRelative" true))))

(fn `MonthlyWeatherChance`
  (returns (WeatherChance_ :type Integer))
  (switch `int` (`/Game/SkyConstruct/Blueprints/BP_SkyConstructMain.Months` (`self.BP_SkyConstructMain`))
    (:`1`
      ;[0 0.5748 1] January
      (return (`|GetArrayItem` (`|MakeArray` 0 1 2 2 3 4 4 4 4 4) (`KismetMathLibrary.RandomIntegerInRange` 0 9))))
    (:`2`
      ;[0.3355 0.8494 1] February
      (return (`|GetArrayItem` (`|MakeArray` 0 0 1 2 2 3 3 4 4 4) (`KismetMathLibrary.RandomIntegerInRange` 0 9))))
    (:`3`
      ;[0.3422 1 0.8799] March
      (return (`|GetArrayItem` (`|MakeArray` 0 0 1 1 1 2 2 3 3 4) (`KismetMathLibrary.RandomIntegerInRange` 0 9))))
    (:`4`
      ;[0.3033 1 0.6336] April
      (return (`|GetArrayItem` (`|MakeArray` 0 0 1 1 1 1 2 2 3 3) (`KismetMathLibrary.RandomIntegerInRange` 0 9))))
    (:`5`
      ;[1 0.7872 0.5462] May
      (return (`|GetArrayItem` (`|MakeArray` 0 0 0 1 1 1 1 2 2 3) (`KismetMathLibrary.RandomIntegerInRange` 0 9))))
    (:`6`
      ;[1 0.5144 0.2656] June
      (return (`|GetArrayItem` (`|MakeArray` 0 0 0 0 1 1 1 1 2 3) (`KismetMathLibrary.RandomIntegerInRange` 0 9))))
    (:`7`
      ;[0.6198 0.274 0.09684] July
      (return (`|GetArrayItem` (`|MakeArray` 0 0 0 0 1 1 1 1 1 2) (`KismetMathLibrary.RandomIntegerInRange` 0 9))))
    (:`8`
      ;[0.4583 0.1616 0.009549] August
      (return (`|GetArrayItem` (`|MakeArray` 0 0 0 0 1 1 1 1 2 3) (`KismetMathLibrary.RandomIntegerInRange` 0 9))))
    (:`9`
      ;[1 0.7299 0.2581] September
      (return (`|GetArrayItem` (`|MakeArray` 0 0 1 1 2 2 2 3 3 3) (`KismetMathLibrary.RandomIntegerInRange` 0 9))))
    (:`10`
      ;[0.6198 0.5554 0.3275] October
      (return (`|GetArrayItem` (`|MakeArray` 0 0 1 1 2 2 3 3 3 3) (`KismetMathLibrary.RandomIntegerInRange` 0 9))))
    (:`11`
      ;[0.405 0.4492 0.4583] November
      (return (`|GetArrayItem` (`|MakeArray` 0 1 1 2 2 3 3 3 4 4) (`KismetMathLibrary.RandomIntegerInRange` 0 9))))
    (:`12`
      ;[0.4031 0.709 1] December
      (return (`|GetArrayItem` (`|MakeArray` 0 0 1 2 2 3 4 4 4 4) (`KismetMathLibrary.RandomIntegerInRange` 0 9))))))

(fn `PartlyCloudyFoggyWeather`
  (params (DeltaTime_ :type "Float (double-precision)"))
  (bind (_partlycloudyfoggyweather_sunintensity _partlycloudyfoggyweather_sunbloomstrength _partlycloudyfoggyweather_bloomscale _partlycloudyfoggyweather_moonintensity _partlycloudyfoggyweather_moonbloomstrength _partlycloudyfoggyweather_moonbloomscale _partlycloudyfoggyweather_skybrightness _partlycloudyfoggyweather_starsbrightness _partlycloudyfoggyweather_skylightintensity _partlycloudyfoggyweather_skylightcolor _partlycloudyfoggyweather_coverage _partlycloudyfoggyweather_lightintensity _partlycloudyfoggyweather_shadowsize _partlycloudyfoggyweather_ambientintensity _partlycloudyfoggyweather_exfogdensity _partlycloudyfoggyweather_foginscolor) (break `/Game/DynamicVolumetricSky/Blueprints/WeatherStructures/PartlyCloudyFoggyWeatherStructure` (`/Game/SkyConstruct/Blueprints/BP_SkyConstructMain.PartlyCloudyFoggyWeather` (`self.BP_SkyConstructMain`))))
  (`self.DifferentWeather` DeltaTime_ (make `/Game/SkyConstruct/Blueprints/WeatherStructures/DifferentWeatherTempStructure` _partlycloudyfoggyweather_sunintensity _partlycloudyfoggyweather_sunbloomstrength _partlycloudyfoggyweather_bloomscale _partlycloudyfoggyweather_moonintensity _partlycloudyfoggyweather_moonbloomstrength _partlycloudyfoggyweather_moonbloomscale _partlycloudyfoggyweather_skybrightness _partlycloudyfoggyweather_starsbrightness _partlycloudyfoggyweather_skylightintensity _partlycloudyfoggyweather_skylightcolor _partlycloudyfoggyweather_coverage 0.0 _partlycloudyfoggyweather_lightintensity _partlycloudyfoggyweather_shadowsize _partlycloudyfoggyweather_ambientintensity _partlycloudyfoggyweather_exfogdensity _partlycloudyfoggyweather_foginscolor))
  (`self.DeactivateRain` DeltaTime_)
  (`self.DeactivateSnow`))

(fn `PartlyCloudyWeather`
  (params (DeltaTime_ :type "Float (double-precision)"))
  (bind (_partlycloudyweather_sunintensity _partlycloudyweather_sunbloomstrength _partlycloudyweather_bloomscale _partlycloudyweather_moonintensity _partlycloudyweather_moonbloomstrength _partlycloudyweather_moonbloomscale _partlycloudyweather_skybrightness _partlycloudyweather_starsbrightness _partlycloudyweather_skylightintensity _partlycloudyweather_skylightcolor _partlycloudyweather_coverage _partlycloudyweather_lightintensity _partlycloudyweather_shadowsize _partlycloudyweather_ambientintensity _partlycloudyweather_exfogdensity _partlycloudyweather_foginscolor) (break `/Game/DynamicVolumetricSky/Blueprints/WeatherStructures/PartlyCloudyWeatherStructure` (`/Game/SkyConstruct/Blueprints/BP_SkyConstructMain.PartlyCloudyWeather` (`self.BP_SkyConstructMain`))))
  (`self.DifferentWeather` DeltaTime_ (make `/Game/SkyConstruct/Blueprints/WeatherStructures/DifferentWeatherTempStructure` _partlycloudyweather_sunintensity _partlycloudyweather_sunbloomstrength _partlycloudyweather_bloomscale _partlycloudyweather_moonintensity _partlycloudyweather_moonbloomstrength _partlycloudyweather_moonbloomscale _partlycloudyweather_skybrightness _partlycloudyweather_starsbrightness _partlycloudyweather_skylightintensity _partlycloudyweather_skylightcolor _partlycloudyweather_coverage 0.0 _partlycloudyweather_lightintensity _partlycloudyweather_shadowsize _partlycloudyweather_ambientintensity _partlycloudyweather_exfogdensity _partlycloudyweather_foginscolor))
  (`self.DeactivateRain` DeltaTime_)
  (`self.DeactivateSnow`))

(fn `RainyFoggyWeather`
  (params (DeltaTime_ :type "Float (double-precision)"))
  (bind (_rainyfoggyweather_sunintensity _rainyfoggyweather_sunbloomstrength _rainyfoggyweather_bloomscale _rainyfoggyweather_moonintensity _rainyfoggyweather_moonbloomstrength _rainyfoggyweather_moonbloomscale _rainyfoggyweather_skybrightness _rainyfoggyweather_starsbrightness _rainyfoggyweather_skylightintensity _rainyfoggyweather_skylightcolor _rainyfoggyweather_coverage _rainyfoggyweather_lightintensity _rainyfoggyweather_shadowsize _rainyfoggyweather_ambientintensity _rainyfoggyweather_exfogdensity _rainyfoggyweather_foginscolor) (break `/Game/DynamicVolumetricSky/Blueprints/WeatherStructures/RainyFoggyWeatherStructureComplicated` (`/Game/SkyConstruct/Blueprints/BP_SkyConstructMain.RainyFoggyWeather` (`self.BP_SkyConstructMain`))))
  (`self.DifferentWeather` DeltaTime_ (make `/Game/SkyConstruct/Blueprints/WeatherStructures/DifferentWeatherTempStructure` _rainyfoggyweather_sunintensity _rainyfoggyweather_sunbloomstrength _rainyfoggyweather_bloomscale _rainyfoggyweather_moonintensity _rainyfoggyweather_moonbloomstrength _rainyfoggyweather_moonbloomscale _rainyfoggyweather_skybrightness _rainyfoggyweather_starsbrightness _rainyfoggyweather_skylightintensity _rainyfoggyweather_skylightcolor _rainyfoggyweather_coverage 0.0 _rainyfoggyweather_lightintensity _rainyfoggyweather_shadowsize _rainyfoggyweather_ambientintensity _rainyfoggyweather_exfogdensity _rainyfoggyweather_foginscolor))
  (`self.ActivateRain` DeltaTime_)
  (`self.DeactivateSnow`))

(fn `RainyWeather`
  (params (DeltaTime_ :type "Float (double-precision)"))
  (bind (_rainyweather_sunintensity _rainyweather_sunbloomstrength _rainyweather_bloomscale _rainyweather_moonintensity _rainyweather_moonbloomstrength _rainyweather_moonbloomscale _rainyweather_skybrightness _rainyweather_starsbrightness _rainyweather_skylightintensity _rainyweather_skylightcolor _rainyweather_coverage _rainyweather_lightintensity _rainyweather_shadowsize _rainyweather_ambientintensity _rainyweather_exfogdensity _rainyweather_foginscolor) (break `/Game/DynamicVolumetricSky/Blueprints/WeatherStructures/RainyWeatherStructure` (`/Game/SkyConstruct/Blueprints/BP_SkyConstructMain.RainyWeather` (`self.BP_SkyConstructMain`))))
  (`self.DifferentWeather` DeltaTime_ (make `/Game/SkyConstruct/Blueprints/WeatherStructures/DifferentWeatherTempStructure` _rainyweather_sunintensity _rainyweather_sunbloomstrength _rainyweather_bloomscale _rainyweather_moonintensity _rainyweather_moonbloomstrength _rainyweather_moonbloomscale _rainyweather_skybrightness _rainyweather_starsbrightness _rainyweather_skylightintensity _rainyweather_skylightcolor _rainyweather_coverage 0.0 _rainyweather_lightintensity _rainyweather_shadowsize _rainyweather_ambientintensity _rainyweather_exfogdensity _rainyweather_foginscolor))
  (`self.ActivateRain` DeltaTime_)
  (`self.DeactivateSnow`))

(fn `SetWindProperties`
  (params (MinWindStrength :type "Float (double-precision)") (MaxWindStrength :type "Float (double-precision)"))
  (bind _returnvalue (* (`/Game/SkyConstruct/Blueprints/BP_SkyConstructMain.WindStrength` (`self.BP_SkyConstructMain`)) (`KismetMathLibrary.Conv_IntToDouble` (`KismetMathLibrary.RandomIntegerInRange` -1 1))))
  (set `/Game/SkyConstruct/Blueprints/BP_SkyConstructMain.WindStrength` (`KismetMathLibrary.RandomFloatInRange` MinWindStrength MaxWindStrength) (`self.BP_SkyConstructMain`))
  (set `/Game/SkyConstruct/Blueprints/BP_SkyConstructMain.CloudWindTarget` (`KismetMathLibrary.MakeColor` _returnvalue _returnvalue -0.01) (`self.BP_SkyConstructMain`))
  (return))

(fn `SnowyFoggyWeather`
  (params (DeltaTime_ :type "Float (double-precision)"))
  (bind (_snowyfoggyweather_sunintensity _snowyfoggyweather_sunbloomstrength _snowyfoggyweather_bloomscale _snowyfoggyweather_moonintensity _snowyfoggyweather_moonbloomstrength _snowyfoggyweather_moonbloomscale _snowyfoggyweather_skybrightness _snowyfoggyweather_starsbrightness _snowyfoggyweather_skylightintensity _snowyfoggyweather_skylightcolor _snowyfoggyweather_coverage _snowyfoggyweather_lightintensity _snowyfoggyweather_shadowsize _snowyfoggyweather_ambientintensity _snowyfoggyweather_exfogdensity _snowyfoggyweather_foginscolor) (break `/Game/DynamicVolumetricSky/Blueprints/WeatherStructures/SnowyFoggyWeatherStructure` (`/Game/SkyConstruct/Blueprints/BP_SkyConstructMain.SnowyFoggyWeather` (`self.BP_SkyConstructMain`))))
  (`self.DifferentWeather` DeltaTime_ (make `/Game/SkyConstruct/Blueprints/WeatherStructures/DifferentWeatherTempStructure` _snowyfoggyweather_sunintensity _snowyfoggyweather_sunbloomstrength _snowyfoggyweather_bloomscale _snowyfoggyweather_moonintensity _snowyfoggyweather_moonbloomstrength _snowyfoggyweather_moonbloomscale _snowyfoggyweather_skybrightness _snowyfoggyweather_starsbrightness _snowyfoggyweather_skylightintensity _snowyfoggyweather_skylightcolor _snowyfoggyweather_coverage 0.0 _snowyfoggyweather_lightintensity _snowyfoggyweather_shadowsize _snowyfoggyweather_ambientintensity _snowyfoggyweather_exfogdensity _snowyfoggyweather_foginscolor))
  (`self.DeactivateRain` DeltaTime_)
  (`self.ActivateSnow`))

(fn `SnowyWeather`
  (params (DeltaTime_ :type "Float (double-precision)"))
  (bind (_snowyweather_sunintensity _snowyweather_sunbloomstrength _snowyweather_bloomscale _snowyweather_moonintensity _snowyweather_moonbloomstrength _snowyweather_moonbloomscale _snowyweather_skybrightness _snowyweather_starsbrightness _snowyweather_skylightintensity _snowyweather_skylightcolor _snowyweather_coverage _snowyweather_lightintensity _snowyweather_shadowsize _snowyweather_ambientintensity _snowyweather_exfogdensity _snowyweather_foginscolor) (break `/Game/DynamicVolumetricSky/Blueprints/WeatherStructures/SnowyWeatherStructure` (`/Game/SkyConstruct/Blueprints/BP_SkyConstructMain.SnowyWeather` (`self.BP_SkyConstructMain`))))
  (`self.DifferentWeather` DeltaTime_ (make `/Game/SkyConstruct/Blueprints/WeatherStructures/DifferentWeatherTempStructure` _snowyweather_sunintensity _snowyweather_sunbloomstrength _snowyweather_bloomscale _snowyweather_moonintensity _snowyweather_moonbloomstrength _snowyweather_moonbloomscale _snowyweather_skybrightness _snowyweather_starsbrightness _snowyweather_skylightintensity _snowyweather_skylightcolor _snowyweather_coverage 0.0 _snowyweather_lightintensity _snowyweather_shadowsize _snowyweather_ambientintensity _snowyweather_exfogdensity _snowyweather_foginscolor))
  (`self.DeactivateRain` DeltaTime_)
  (`self.ActivateSnow`))

(fn `SunnyFoggyWeather`
  (params (DeltaTime_ :type "Float (double-precision)"))
  (bind (_sunnyfoggyweather_sunintensity _sunnyfoggyweather_sunbloomstrength _sunnyfoggyweather_bloomscale _sunnyfoggyweather_moonintensity _sunnyfoggyweather_moonbloomstrength _sunnyfoggyweather_moonbloomscale _sunnyfoggyweather_skybrightness _sunnyfoggyweather_starsbrightness _sunnyfoggyweather_skylightintensity _sunnyfoggyweather_skylightcolor _sunnyfoggyweather_coverage _sunnyfoggyweather_lightintensity _sunnyfoggyweather_shadowsize _sunnyfoggyweather_ambientintensity _sunnyfoggyweather_exfogdensity _sunnyfoggyweather_foginscolor) (break `/Game/DynamicVolumetricSky/Blueprints/WeatherStructures/SunnyFoggyWeatherStructure` (`/Game/SkyConstruct/Blueprints/BP_SkyConstructMain.SunnyFoggyWeather` (`self.BP_SkyConstructMain`))))
  (`self.DifferentWeather` DeltaTime_ (make `/Game/SkyConstruct/Blueprints/WeatherStructures/DifferentWeatherTempStructure` _sunnyfoggyweather_sunintensity _sunnyfoggyweather_sunbloomstrength _sunnyfoggyweather_bloomscale _sunnyfoggyweather_moonintensity _sunnyfoggyweather_moonbloomstrength _sunnyfoggyweather_moonbloomscale _sunnyfoggyweather_skybrightness _sunnyfoggyweather_starsbrightness _sunnyfoggyweather_skylightintensity _sunnyfoggyweather_skylightcolor _sunnyfoggyweather_coverage 0.0 _sunnyfoggyweather_lightintensity _sunnyfoggyweather_shadowsize _sunnyfoggyweather_ambientintensity _sunnyfoggyweather_exfogdensity _sunnyfoggyweather_foginscolor))
  (`self.DeactivateRain` DeltaTime_)
  (`self.DeactivateSnow`))

(fn `SunnyWeather`
  (params (DeltaTime_ :type "Float (double-precision)"))
  (bind (_sunnyweather_sunintensity _sunnyweather_sunbloomstrength _sunnyweather_bloomscale _sunnyweather_moonintensity _sunnyweather_moonbloomstrength _sunnyweather_moonbloomscale _sunnyweather_skybrightness _sunnyweather_starsbrightness _sunnyweather_skylightintensity _sunnyweather_skylightcolor _sunnyweather_coverage _sunnyweather_lightintensity _sunnyweather_shadowsize _sunnyweather_ambientintensity _sunnyweather_exfogdensity _sunnyweather_foginscolor) (break `/Game/DynamicVolumetricSky/Blueprints/WeatherStructures/SunnyWeatherStructure` (`/Game/SkyConstruct/Blueprints/BP_SkyConstructMain.SunnyWeather` (`self.BP_SkyConstructMain`))))
  (`self.DifferentWeather` DeltaTime_ (make `/Game/SkyConstruct/Blueprints/WeatherStructures/DifferentWeatherTempStructure` _sunnyweather_sunintensity _sunnyweather_sunbloomstrength _sunnyweather_bloomscale _sunnyweather_moonintensity _sunnyweather_moonbloomstrength _sunnyweather_moonbloomscale _sunnyweather_skybrightness _sunnyweather_starsbrightness _sunnyweather_skylightintensity _sunnyweather_skylightcolor _sunnyweather_coverage 0.0 _sunnyweather_lightintensity _sunnyweather_shadowsize _sunnyweather_ambientintensity _sunnyweather_exfogdensity _sunnyweather_foginscolor))
  (`self.DeactivateRain` DeltaTime_)
  (`self.DeactivateSnow`))