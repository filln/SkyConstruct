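; BP_Rain is a rain effect actor that follows the player camera via an attached spring arm.
; Init creates rain and splash dynamic materials, randomizes particle forces, fades in the sound and runs a looping timer that ramps spawn rate to a random maximum.
; Stop fades the sound out and ramps the spawn rate down on the same timer handle, destroying the actor at zero.
; Init runs from both the construction script and BeginPlay.
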(event `self.ReceiveBeginPlay`
  (`self.Init`))

(fn `DecreaseSpawnRate`
  (bind _bp_rain_ps (`self.BP_Rain_PS`))
  (bind _spawnrate (`self.SpawnRate`))
  (set `self.SpawnRate` (`KismetMathLibrary.FInterpTo_Constant` (`self.SpawnRate`) 0.0 (`self.SpawnRateDeltaTime`) (`self.SpawnRateSpeed`)))
  (`ParticleSystemComponent.SetFloatParameter` _bp_rain_ps "SpawnRate" _spawnrate)
  (`ParticleSystemComponent.SetFloatParameter` _bp_rain_ps "SpawnRate2" (* _spawnrate 5.0))
  (if (<= (`self.SpawnRate`) 0.0)
    (`KismetSystemLibrary.K2_ClearAndInvalidateTimerHandle` (`self.SpawnRateTimer`))
    (`self.K2_DestroyActor`)))

(fn `IncreaseSpawnRate`
  (bind _bp_rain_ps (`self.BP_Rain_PS`))
  (bind _spawnrate (`self.SpawnRate`))
  (set `self.SpawnRate` (`KismetMathLibrary.FInterpTo_Constant` (`self.SpawnRate`) (`self.MaxRandomSpawnRate`) (`self.SpawnRateDeltaTime`) (`self.SpawnRateSpeed`)))
  (`ParticleSystemComponent.SetFloatParameter` _bp_rain_ps "SpawnRate" _spawnrate)
  (`ParticleSystemComponent.SetFloatParameter` _bp_rain_ps "SpawnRate2" (* _spawnrate 5.0))
  (if (>= (`self.SpawnRate`) (`self.MaxRandomSpawnRate`))
    (`KismetSystemLibrary.K2_ClearAndInvalidateTimerHandle` (`self.SpawnRateTimer`))))

(fn `Init`
  (set `self.MaxRandomSpawnRate` (`KismetMathLibrary.RandomFloatInRange` (`self.MaxSpawnRateMin`) (`self.MaxSpawnRateMax`)))
  (set `self.SpawnRateSpeed` (/ (`self.MaxRandomSpawnRate`) (`self.SpawnRateTime`)))
  (set `self.SoundFadeDuration` (/ (`self.MaxRandomSpawnRate`) (`self.SpawnRateSpeed`)))
  (`KismetSystemLibrary.K2_ClearAndInvalidateTimerHandle` (`self.SpawnRateTimer`))
  (bind _returnvalue (`KismetSystemLibrary.K2_SetTimer` null "IncreaseSpawnRate" (`self.SpawnRateDeltaTime`) true))
  (set `self.SpawnRateTimer` _returnvalue)
  (`self.MaterialFunctionality`)
  (`AudioComponent.FadeIn` (`self.RainSound`) (`self.SoundFadeDuration`) 1.0 0.0 "Linear")
  (`SceneComponent.K2_AttachToComponent` (`self.RainSpringARM`) (`PlayerCameraManager.TransformComponent` (`GameplayStatics.GetPlayerCameraManager` 0)) "None" "KeepRelative" "KeepRelative" "KeepRelative" true))

(fn `MaterialFunctionality`
  (bind _returnvalue (`KismetMathLibrary.RandomFloatInRange` 0.5 1.5))
  (bind _returnvalue_2 (`KismetMaterialLibrary.CreateDynamicMaterialInstance` "/Game/SkyConstruct/Materials/ParticleMaterials/Rain/RainDrop_Inst.RainDrop_Inst"))
  (set `self.RainMat` _returnvalue_2)
  (`PrimitiveComponent.SetMaterial` (`self.BP_Rain_PS`) 0 (`self.RainMat`))
  (`PrimitiveComponent.SetMaterial` (`self.BP_Rain_PS`) 2 (`self.RainMat`))
  (bind _returnvalue_3 (`PrimitiveComponent.CreateDynamicMaterialInstance` (`self.BP_Rain_PS`) 1 "/Game/SkyConstruct/Materials/ParticleMaterials/Rain/Splash_Inst.Splash_Inst" "None"))
  (set `self.SplashMat` _returnvalue_3)
  (`ParticleSystemComponent.SetVectorParameter` (`self.BP_Rain_PS`) "Forces" (`KismetMathLibrary.MakeVector` (* (.x (`self.Forces`)) _returnvalue) (* (.y (`self.Forces`)) _returnvalue) (* (.z (`self.Forces`)) (`KismetMathLibrary.RandomFloatInRange` 0.75 1.25))))
  (`MaterialInstanceDynamic.SetVectorParameterValue` (`self.RainMat`) "RainColor" (`self.RainColor`))
  (`MaterialInstanceDynamic.SetScalarParameterValue` (`self.RainMat`) "Emissive" (`self.Emissive`))
  (`MaterialInstanceDynamic.SetScalarParameterValue` (`self.RainMat`) "RainOpacity" (`self.Opacity`))
  (`MaterialInstanceDynamic.SetScalarParameterValue` (`self.RainMat`) "RainDistortion" (`self.Distortion`))
  (`MaterialInstanceDynamic.SetVectorParameterValue` (`self.SplashMat`) "LiquidColor" (`self.RainColor`))
  (`MaterialInstanceDynamic.SetScalarParameterValue` (`self.SplashMat`) "Emissive" (`self.Emissive`))
  (`MaterialInstanceDynamic.SetScalarParameterValue` (`self.SplashMat`) "Opacity" (* (`self.Opacity`) 0.5)))

(fn `Stop`
  (`AudioComponent.FadeOut` (`self.RainSound`) (`self.SoundFadeDuration`) 0.0 "Linear")
  (`KismetSystemLibrary.K2_ClearAndInvalidateTimerHandle` (`self.SpawnRateTimer`))
  (bind _returnvalue (`KismetSystemLibrary.K2_SetTimer` null "DecreaseSpawnRate" (`self.SpawnRateDeltaTime`) true))
  (set `self.SpawnRateTimer` _returnvalue))

(fn `UserConstructionScript`
  (`self.Init`))