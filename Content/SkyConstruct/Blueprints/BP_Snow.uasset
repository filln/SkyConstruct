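; BP_Snow is a weather actor that renders camera-following snowfall through a particle effect on a spring arm attached to the player camera manager.
; BeginPlay polls until the weather manager's sky reference is valid, then runs Init, which ramps spawn rate toward a randomized maximum.
; A looping timer keeps randomizing flake size and force strength.
; Stop ramps spawn rate down to zero, then destroys the actor; wind-based rotation is present but unconnected.
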(event `self.ReceiveBeginPlay`
  (`/Game/SkyConstruct/Blueprints/CoreClasses/BeginPlayInterface.StartBeginPlayTimer`))

(event `/Game/SkyConstruct/Blueprints/CoreClasses/BeginPlayInterface.DoBeginPlay`
  (set `self.BP_SkyConstructMain` (`/Game/SkyConstruct/Blueprints/BP_WeatherManager.BP_SkyConstructMain` (`/Game/SkyConstruct/Blueprints/CoreClasses/ScyConstructGameMode.BP_WeatherManager` (cast `/Game/SkyConstruct/Blueprints/CoreClasses/ScyConstructGameMode` (`GameplayStatics.GetGameMode`) :!pure true))))
  (`self.Init`)
  (`KismetSystemLibrary.K2_SetTimerDelegate` (delegate `MainTimer`) 0.1 true))

(event `MainTimer`
  (bind _returnvalue (`KismetMathLibrary.RandomFloatInRange` (`self.FlakeSizeSmall`) (`self.FlakeSizeLarge`)))
  (`ParticleSystemComponent.SetVectorParameter` (`self.VFX_Weather_Snow_ForBP`) "FlakeSize" (`KismetMathLibrary.MakeVector` _returnvalue _returnvalue _returnvalue))
  (`ParticleSystemComponent.SetVectorParameter` (`self.VFX_Weather_Snow_ForBP`) "Forces" (* (`self.Forces`) (`KismetMathLibrary.RandomFloatInRange` 0.5 1.5))))

(event `/Game/SkyConstruct/Blueprints/CoreClasses/BeginPlayInterface.BeforeBeginPlay`
  (bind _isvalid (`/Game/SkyConstruct/Blueprints/CoreClasses/BeginPlayInterface.CheckReferences`))
  (if _isvalid
    (`/Game/SkyConstruct/Blueprints/CoreClasses/BeginPlayInterface.DoBeginPlay`)
    (`KismetSystemLibrary.K2_ClearAndInvalidateTimerHandle` (`self.BeginPlayTimer`))))

(event `/Game/SkyConstruct/Blueprints/CoreClasses/BeginPlayInterface.StartBeginPlayTimer`
  (bind _returnvalue (`KismetSystemLibrary.K2_SetTimerDelegate` (delegate `/Game/SkyConstruct/Blueprints/CoreClasses/BeginPlayInterface.BeforeBeginPlay`) 0.2 true))
  (set `self.BeginPlayTimer` _returnvalue))

(fn `CheckReferences`
  (returns (IsValid :type Boolean))
  (bind _asscy_construct_game_mode (cast `/Game/SkyConstruct/Blueprints/CoreClasses/ScyConstructGameMode` (`GameplayStatics.GetGameMode`))
    (:`then`
      (bind _bp_weathermanager (`/Game/SkyConstruct/Blueprints/CoreClasses/ScyConstructGameMode.BP_WeatherManager` _asscy_construct_game_mode))
      (`/Engine/EditorBlueprintResources/StandardMacros.IsValid` _bp_weathermanager
        (:`Is Valid`
          (return (`KismetSystemLibrary.IsValid` (`/Game/SkyConstruct/Blueprints/BP_WeatherManager.BP_SkyConstructMain` _bp_weathermanager))))
        (:`Is Not Valid`
          (return false))))
    (:`CastFailed`
      (return false))))

(fn `DecreaseSpawnRate`
  (set `self.SpawnRate` (`KismetMathLibrary.FInterpTo_Constant` (`self.SpawnRate`) 0.0 (`self.SpawnRateDeltaTime`) (`self.SpawnRateSpeed`)))
  (`ParticleSystemComponent.SetFloatParameter` (`self.VFX_Weather_Snow_ForBP`) "SpawnRate" (`self.SpawnRate`))
  (if (<= (`self.SpawnRate`) 0.0)
    (`KismetSystemLibrary.K2_ClearAndInvalidateTimerHandle` (`self.SpawnRateTimer`))
    (`self.K2_DestroyActor`)))

(fn `IncreaseSpawnRate`
  (set `self.SpawnRate` (`KismetMathLibrary.FInterpTo_Constant` (`self.SpawnRate`) (`self.MaxRandomSpawnRate`) (`self.SpawnRateDeltaTime`) (`self.SpawnRateSpeed`)))
  (`ParticleSystemComponent.SetFloatParameter` (`self.VFX_Weather_Snow_ForBP`) "SpawnRate" (`self.SpawnRate`))
  (if (>= (`self.SpawnRate`) (`self.MaxRandomSpawnRate`))
    (`KismetSystemLibrary.K2_ClearAndInvalidateTimerHandle` (`self.SpawnRateTimer`))))

(fn `Init`
  (set `self.MaxRandomSpawnRate` (`KismetMathLibrary.RandomFloatInRange` (`self.MaxSpawnRateMin`) (`self.MaxSpawnRateMax`)))
  (set `self.SpawnRateSpeed` (/ (`self.MaxRandomSpawnRate`) (`self.SpawnRateTime`)))
  (`KismetSystemLibrary.K2_ClearAndInvalidateTimerHandle` (`self.SpawnRateTimer`))
  (bind _returnvalue (`KismetSystemLibrary.K2_SetTimer` null "IncreaseSpawnRate" (`self.SpawnRateDeltaTime`) true))
  (set `self.SpawnRateTimer` _returnvalue)
  (`self.MaterialFunctionality`)
  (`SceneComponent.K2_AttachToComponent` (`self.SnowSpringARM`) (`PlayerCameraManager.TransformComponent` (`GameplayStatics.GetPlayerCameraManager` 0)) "None" "KeepRelative" "KeepRelative" "KeepRelative" true))

(fn `MaterialFunctionality`
  (bind _returnvalue (`KismetMathLibrary.RandomFloatInRange` (`self.FlakeSizeSmall`) (`self.FlakeSizeLarge`)))
  (`ParticleSystemComponent.SetVectorParameter` (`self.VFX_Weather_Snow_ForBP`) "FlakeSize" (`KismetMathLibrary.MakeVector` _returnvalue _returnvalue _returnvalue))
  (`ParticleSystemComponent.SetVectorParameter` (`self.VFX_Weather_Snow_ForBP`) "Forces" (* (`self.Forces`) (`KismetMathLibrary.RandomFloatInRange` 0.5 1.5))))

(fn `Stop`
  (`KismetSystemLibrary.K2_ClearAndInvalidateTimerHandle` (`self.SpawnRateTimer`))
  (bind _returnvalue (`KismetSystemLibrary.K2_SetTimer` null "DecreaseSpawnRate" (`self.SpawnRateDeltaTime`) true))
  (set `self.SpawnRateTimer` _returnvalue))

(fn `UserConstructionScript`
  (`self.Init`))