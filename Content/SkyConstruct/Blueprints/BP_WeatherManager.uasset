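; Weather manager Blueprint that registers itself with the game mode and drives global rain wetness for materials.
; Activation and deactivation calls from a dynamic weather actor fire rain events and set wetness and raindrop parameters in MPC_Weather.
; Timelines fade wetness in and out, sharing a stored playback position to handle interrupted transitions.
; Only the weather actor that activated wetness can deactivate it, and effect flags clear when the fade-out finishes.
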(event `self.ReceiveBeginPlay`
  (bind _asscy_construct_game_mode (cast `/Game/SkyConstruct/Blueprints/CoreClasses/ScyConstructGameMode` (`GameplayStatics.GetGameMode`)))
  (set `/Game/SkyConstruct/Blueprints/CoreClasses/ScyConstructGameMode.BP_WeatherManager` self _asscy_construct_game_mode))

(event `ActivateWetness`
  (params (BP_DynamicWeather :type "ActorComponent Object Reference"))
  (if (not (`self.isWetnessActivated`))
    (set `self.isWetnessActivated` true)
    (set `self.BP_DynamicWeatherTmp` BP_DynamicWeather)
    (`self.OnRainActivated`)
    (`KismetMaterialLibrary.SetScalarParameterValue` "/Game/SkyConstruct/Materials/MaterialParameterCollections/MPC_Weather.MPC_Weather" "isRunWetness" 1.0)
    (`KismetMaterialLibrary.SetScalarParameterValue` "/Game/SkyConstruct/Materials/MaterialParameterCollections/MPC_Weather.MPC_Weather" "isRunRainDrop" 1.0)
    (`KismetMaterialLibrary.SetScalarParameterValue` "/Game/SkyConstruct/Materials/MaterialParameterCollections/MPC_Weather.MPC_Weather" "SpeedOfAnimateRainDrop" (`self.MaxSpeedOfAnimateRainDrop`))
    (bind (_direction _fc_wetness _playbackposition) (`Timeline|Wetness` :`NewTime` (`self.WetnessPlaybackPosition`))
      (:`Update`
        (set `self.WetnessPlaybackPosition` _playbackposition)
        (bind _output_get (set `self.GlobalWetness` _fc_wetness))
        (`KismetMaterialLibrary.SetScalarParameterValue` "/Game/SkyConstruct/Materials/MaterialParameterCollections/MPC_Weather.MPC_Weather" "GlobalWetness" _output_get)
        (`KismetMaterialLibrary.SetScalarParameterValue` "/Game/SkyConstruct/Materials/MaterialParameterCollections/MPC_Weather.MPC_Weather" "GlobalRainDrop" _output_get)))))

(event `DeactivateWetness`
  (params (BP_DynamicWeather :type "ActorComponent Object Reference"))
  (if (== BP_DynamicWeather (`self.BP_DynamicWeatherTmp`))
    (set `self.isWetnessActivated` false)
    (`self.OnRainDeactivated`)
    (`KismetMaterialLibrary.SetScalarParameterValue` "/Game/SkyConstruct/Materials/MaterialParameterCollections/MPC_Weather.MPC_Weather" "SpeedOfAnimateRainDrop" (`self.MinSpeedOfAnimateRainDrop`))
    (bind (_direction _fc_wetness _playbackposition) (`Timeline|WetnessReverse` :`NewTime` (`self.WetnessPlaybackPosition`) :!via `ReverseFromEnd`)
      (:`Update`
        (set `self.WetnessPlaybackPosition` _playbackposition)
        (bind _output_get (set `self.GlobalWetness` _fc_wetness))
        (`KismetMaterialLibrary.SetScalarParameterValue` "/Game/SkyConstruct/Materials/MaterialParameterCollections/MPC_Weather.MPC_Weather" "GlobalWetness" _output_get)
        (`KismetMaterialLibrary.SetScalarParameterValue` "/Game/SkyConstruct/Materials/MaterialParameterCollections/MPC_Weather.MPC_Weather" "GlobalRainDrop" _output_get))
      (:`Finished`
        (`KismetMaterialLibrary.SetScalarParameterValue` "/Game/SkyConstruct/Materials/MaterialParameterCollections/MPC_Weather.MPC_Weather" "isRunWetness" 0.0)
        (`KismetMaterialLibrary.SetScalarParameterValue` "/Game/SkyConstruct/Materials/MaterialParameterCollections/MPC_Weather.MPC_Weather" "isRunRainDrop")))))

(fn `UserConstructionScript`)