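; Component that applies Low, Medium, High or Epic quality presets to the volumetric cloud and fog settings of its owning BP_SkyConstructMain.
; BeginPlay caches the owner and starts a looping timer that polls CheckSetttings instead of using Tick.
; When simple settings are enabled, an ApplySettings flag or a changed preset enum triggers SwitchSettings.
; The selected preset's values are copied onto the sky actor through SetDifferent.
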(event `self.ReceiveBeginPlay`
  (set `self.BP_SkyConstructMain` (cast `/Game/SkyConstruct/Blueprints/BP_SkyConstructMain` (`self.GetOwner`) :!pure true))
  (`KismetSystemLibrary.K2_SetTimer` null "CheckSetttings" (`self.CheckSetttingsDeltaTime`) true))

(fn `CheckSetttings`
  (if (`self.IsUseSimpleSettings`)
    (if (`self.ApplySettings`)
      (set `self.ApplySettings` false)
      (`self.SwitchSettings` (`self.ESkySimpleSettings`))
      (return)
      (elif (`|EnumEquality` (`self.ESkySimpleSettings`) (`self.ESkySimpleSettingsTmp`))
        (return)
        (else
          (set `self.ESkySimpleSettingsTmp` (`self.ESkySimpleSettings`))
          (`self.SwitchSettings` (`self.ESkySimpleSettings`))
          (return))))
    (else
      (return))))

(fn `SetDifferent`
  (params (_InputSettings :type "/Game/SkyConstruct/Blueprints/SimpleSettings/InputTmpSkySettingsStruct Structure"))
  (set `/Game/SkyConstruct/Blueprints/BP_SkyConstructMain.ReversedRaymarchStep` _InputSettings_ReversedRaymarchStep_4_476892B241B4BFA80B7BE495788933F8 (`self.BP_SkyConstructMain`))
  (set `/Game/SkyConstruct/Blueprints/BP_SkyConstructMain.StepDistanceScale` _InputSettings_StepDistanceScale_5_7F1794054813BF136009AF8E0AE9183C (`self.BP_SkyConstructMain`))
  (set `/Game/SkyConstruct/Blueprints/BP_SkyConstructMain.CloudTopOffset` _InputSettings_CloudTopOffset_11_3F104BB44E3D3C004FBDF2A2941E58FD (`self.BP_SkyConstructMain`))
  (set `/Game/SkyConstruct/Blueprints/BP_SkyConstructMain.WeatherTile` _InputSettings_WeatherTile_13_66E5F9264723264A6F7DF5A325CD1C04 (`self.BP_SkyConstructMain`))
  (set `/Game/SkyConstruct/Blueprints/BP_SkyConstructMain.DensityTAA` _InputSettings_DensityTAA_25_332FC67644E521E7AAF614B6BD9C0725 (`self.BP_SkyConstructMain`))
  (set `/Game/SkyConstruct/Blueprints/BP_SkyConstructMain.LightMarchStep` _InputSettings_LightMarchStep_27_C2B4A58F4DD85B74B12B6399F4141DD4 (`self.BP_SkyConstructMain`))
  (set `/Game/SkyConstruct/Blueprints/BP_SkyConstructMain.VolumetricFogEnable?` `_InputSettings_VolumetricFogEnable?_70_4A64AB3F4035089D9FBFBF948B430FEB` (`self.BP_SkyConstructMain`))
  (return))

(fn `SetEpic`
  (bind (_epic_reversedraymarchstep _epic_stepdistancescale _epic_cloudtopoffset _epic_weathertile _epic_densitytaa _epic_lightmarchstep _epic_volumetricfogenable_) (break `/Game/SkyConstruct/Blueprints/SimpleSettings/EpicSkySettingsStruct` (`self.Epic`)))
  (`self.SetDifferent` (make `/Game/SkyConstruct/Blueprints/SimpleSettings/InputTmpSkySettingsStruct` _epic_reversedraymarchstep _epic_stepdistancescale _epic_cloudtopoffset _epic_weathertile _epic_densitytaa _epic_lightmarchstep _epic_volumetricfogenable_)))

(fn `SetHigh`
  (bind (_high_reversedraymarchstep _high_stepdistancescale _high_cloudtopoffset _high_weathertile _high_densitytaa _high_lightmarchstep _high_volumetricfogenable_) (break `/Game/SkyConstruct/Blueprints/SimpleSettings/HighSkySettingsStruct` (`self.High`)))
  (`self.SetDifferent` (make `/Game/SkyConstruct/Blueprints/SimpleSettings/InputTmpSkySettingsStruct` _high_reversedraymarchstep _high_stepdistancescale _high_cloudtopoffset _high_weathertile _high_densitytaa _high_lightmarchstep _high_volumetricfogenable_)))

(fn `SetLow`
  (bind (_low_reversedraymarchstep _low_stepdistancescale _low_cloudtopoffset _low_weathertile _low_densitytaa _low_lightmarchstep _low_volumetricfogenable_) (break `/Game/SkyConstruct/Blueprints/SimpleSettings/LowSkySettingsStruct` (`self.Low`)))
  (`self.SetDifferent` (make `/Game/SkyConstruct/Blueprints/SimpleSettings/InputTmpSkySettingsStruct` _low_reversedraymarchstep _low_stepdistancescale _low_cloudtopoffset _low_weathertile _low_densitytaa _low_lightmarchstep _low_volumetricfogenable_)))

(fn `SetMedium`
  (bind (_medium_reversedraymarchstep _medium_stepdistancescale _medium_cloudtopoffset _medium_weathertile _medium_densitytaa _medium_lightmarchstep _medium_volumetricfogenable_) (break `/Game/SkyConstruct/Blueprints/SimpleSettings/MediumSkySettingsStruct` (`self.Medium`)))
  (`self.SetDifferent` (make `/Game/SkyConstruct/Blueprints/SimpleSettings/InputTmpSkySettingsStruct` _medium_reversedraymarchstep _medium_stepdistancescale _medium_cloudtopoffset _medium_weathertile _medium_densitytaa _medium_lightmarchstep _medium_volumetricfogenable_)))

(fn `SwitchSettings`
  (params (_ESkySimpleSettings :type "/Game/SkyConstruct/Blueprints/Enums/ESkySimpleSettings Enum" :default "NewEnumerator0"))
  (switch `/Game/SkyConstruct/Blueprints/Enums/ESkySimpleSettings` _ESkySimpleSettings
    (:`NewEnumerator0`
      (`self.SetLow`))
    (:`NewEnumerator1`
      (`self.SetMedium`))
    (:`NewEnumerator2`
      (`self.SetHigh`))
    (:`NewEnumerator3`
      (`self.SetEpic`))))