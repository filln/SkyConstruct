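; Parent Blueprint for SkyConstruct test actors that need the weather manager, with empty rain activated and deactivated events.
; On BeginPlay, a looping timer polls until the ScyConstructGameMode holds a valid BPWeatherManager.
; It then caches that manager, calls the empty AssignDispatchers hook and clears the timer, deferring setup until the reference exists.
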(event `self.ReceiveBeginPlay`
  (`self.StartBeginPlayTimer`))

(event `AssignDispatchers`)

(event `RainActivated`)

(event `RainDeactivated`)

(fn `BeforeBeginPlay`
  (if (`self.CheckReferences`)
    (`self.DoBeginPlay`)
    (`KismetSystemLibrary.K2_ClearAndInvalidateTimerHandle` (`self.BeginPlayTimer`))
    (return)
    (else
      (return))))

(fn `CheckReferences`
  (returns (IsValid :type Boolean))
  (bind _asscy_construct_game_mode (cast `/Game/SkyConstruct/Blueprints/CoreClasses/ScyConstructGameMode` (`GameplayStatics.GetGameMode`))
    (:`then`
      (return (`KismetSystemLibrary.IsValid` (`/Game/SkyConstruct/Blueprints/CoreClasses/ScyConstructGameMode.BP_WeatherManager` _asscy_construct_game_mode))))
    (:`CastFailed`
      (return false))))

(fn `DoBeginPlay`
  (bind _asscy_construct_game_mode (cast `/Game/SkyConstruct/Blueprints/CoreClasses/ScyConstructGameMode` (`GameplayStatics.GetGameMode`)))
  (set `self.BP_WeatherManager` (`/Game/SkyConstruct/Blueprints/CoreClasses/ScyConstructGameMode.BP_WeatherManager` _asscy_construct_game_mode))
  (`self.AssignDispatchers`))

(fn `StartBeginPlayTimer`
  (bind _returnvalue (`KismetSystemLibrary.K2_SetTimer` null "BeforeBeginPlay" (`self.BeginPlayDeltaTime`) true))
  (set `self.BeginPlayTimer` _returnvalue))

(fn `UserConstructionScript`)