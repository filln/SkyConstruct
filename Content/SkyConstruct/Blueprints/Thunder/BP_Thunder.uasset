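; BP_Thunder is a Sky Construct thunder spawner that creates BP_ThunderBolt lightning strikes around the player pawn.
; SetStartThunderTimer arms a one-shot, random-delay timer for StartThunder, which spawns a bolt if thunder is possible and passes it a self reference.
; Strike locations use random per-axis offsets, with SignedClamp enforcing minimum and maximum distance in either direction, at a set height.
; CalcMaxStrikeDistance exposes the farthest possible strike distance from the player.
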(event `self.ReceiveBeginPlay`)

(fn `CalcMaxStrikeDistance`
  (returns (MaxStrikeDistance_ :type "Float (double-precision)"))
  (locals (PlayerLocationLoc :type "Vector Structure" :default (0.0 0.0 0.0)))
  (bind (_playerlocationloc_x _playerlocationloc_y) (`KismetMathLibrary.BreakVector` (`local.PlayerLocationLoc`)))
  (set `local.PlayerLocationLoc` (`Actor.K2_GetActorLocation` (`GameplayStatics.GetPlayerPawn` 0)))
  (return (`KismetMathLibrary.VSize` (- (`KismetMathLibrary.MakeVector` (+ (`self.Lightning Max X Distance from Pawn`) _playerlocationloc_x) (+ (`self.Lightning Max Y Distance from Pawn`) _playerlocationloc_y) (`self.Lightning Z Distance from Origin`)) (`local.PlayerLocationLoc`)))))

(fn `CalcStrikeLocation`
  (returns (StrikeLocation :type "Vector Structure"))
  (locals (RandomXLoc :type "Float (double-precision)" :default 0.0) (RandomYLoc :type "Float (double-precision)" :default 0.0) (ClampedXLoc :type "Float (double-precision)" :default 0.0))
  (bind _lightning_max_x_distance_from_pawn (`self.Lightning Max X Distance from Pawn`))
  (bind _lightning_max_y_distance_from_pawn (`self.Lightning Max Y Distance from Pawn`))
  (bind (_returnvalue_x _returnvalue_y) (`KismetMathLibrary.BreakVector` (`Actor.K2_GetActorLocation` (`GameplayStatics.GetPlayerPawn` 0))))
  (set `local.RandomXLoc` (`KismetMathLibrary.RandomFloatInRange` (* _lightning_max_x_distance_from_pawn -1.0) _lightning_max_x_distance_from_pawn))
  (set `local.RandomYLoc` (`KismetMathLibrary.RandomFloatInRange` (* _lightning_max_y_distance_from_pawn -1.0) _lightning_max_y_distance_from_pawn))
  (return (`KismetMathLibrary.MakeVector` (+ (`self.SignedClamp` (`local.RandomXLoc`) (`self.Lightning Min X Distance from Pawn`) (`self.Lightning Max X Distance from Pawn`)) _returnvalue_x) (+ (`self.SignedClamp` (`local.RandomYLoc`) (`self.Lightning Min Y Distance from Pawn`) (`self.Lightning Max Y Distance from Pawn`)) _returnvalue_y) (`self.Lightning Z Distance from Origin`))))

(fn `ClearStartThunderTimer`
  (`KismetSystemLibrary.K2_ClearAndInvalidateTimerHandle` (`self.StartThunderTimer`)))

(fn `SetStartThunderTimer`
  (if (`KismetSystemLibrary.K2_IsTimerActiveHandle` (`self.StartThunderTimer`))
    (return)
    (else
      (bind _returnvalue (`KismetSystemLibrary.K2_SetTimer` null "StartThunder" (`KismetMathLibrary.RandomFloatInRange` (`self.DelayMinStartThunder`) (`self.DelayMaxStartThunder`))))
      (set `self.StartThunderTimer` _returnvalue)
      (return))))

(fn `SignedClamp`
  (params (Value_ :type "Float (double-precision)") (Min_ :type "Float (double-precision)") (Max_ :type "Float (double-precision)"))
  (returns (ReturnValue_ :type "Float (double-precision)"))
  (locals (Value :type "Float (double-precision)") (Min :type "Float (double-precision)" :default 0.0) (Max :type "Float (double-precision)" :default 1.0))
  (set `local.Value` Value_)
  (set `local.Min` Min_)
  (set `local.Max` Max_)
  (if (> (`local.Value`) 0.0)
    (return (`KismetMathLibrary.FClamp` (`local.Value`) (`local.Min`) (`local.Max`)))
    (elif (< (`local.Value`) 0.0)
      (return (* (`KismetMathLibrary.FClamp` (* (`local.Value`) -1.0) (`local.Min`) (`local.Max`)) -1.0))
      (else
        (return (`local.Min`))))))

(fn `StartThunder`
  (if (`self.isThunderPossible`)
    (set `self.StrikeLocation` (`self.CalcStrikeLocation`))
    (bind _returnvalue (`|SpawnActorFromClass` "/Game/SkyConstruct/Blueprints/Thunder/BP_ThunderBolt.BP_ThunderBolt_C" (`KismetMathLibrary.MakeTransform` (`self.StrikeLocation`) (struct) (`self.ThunderBoltScale`)) "AlwaysSpawn" "OverrideRootScale" null null))
    (set `/Game/SkyConstruct/Blueprints/Thunder/BP_ThunderBolt.BP_Thunder` self _returnvalue)
    (return)
    (else
      (return))))