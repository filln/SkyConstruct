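; Lightning bolt actor that shows a randomized strike particle and plays distance-based thunder, using strike data from a BPThunder reference.
; A looping timer polls until that reference is valid, then picks a random particle template and material.
; Timers activate the particle, optionally repeating, and deactivate it after a random delay.
; Player pawn distance selects immediate near or delayed far or very far sound, whose completion destroys the actor.
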(event `self.ReceiveBeginPlay`
  (`/Game/SkyConstruct/Blueprints/CoreClasses/BeginPlayInterface.StartBeginPlayTimer`))

(event `/Game/SkyConstruct/Blueprints/CoreClasses/BeginPlayInterface.BeforeBeginPlay`
  (bind _isvalid (`/Game/SkyConstruct/Blueprints/CoreClasses/BeginPlayInterface.CheckReferences`))
  (if _isvalid
    (`/Game/SkyConstruct/Blueprints/CoreClasses/BeginPlayInterface.DoBeginPlay`)
    (`KismetSystemLibrary.K2_ClearAndInvalidateTimerHandle` (`self.BeginPlayTimer`))))

(event `/Game/SkyConstruct/Blueprints/CoreClasses/BeginPlayInterface.StartBeginPlayTimer`
  (bind _returnvalue (`KismetSystemLibrary.K2_SetTimerDelegate` (delegate `/Game/SkyConstruct/Blueprints/CoreClasses/BeginPlayInterface.BeforeBeginPlay`) 0.02 true))
  (set `self.BeginPlayTimer` _returnvalue))

(event `/Game/SkyConstruct/Blueprints/CoreClasses/BeginPlayInterface.DoBeginPlay`
  (`self.MaterialFunctionality`)
  (bind _returnvalue (`KismetSystemLibrary.K2_SetTimer` null "CastLightning" (`self.DelayCastLightning`) (`self.isRepeatLightning`)))
  (set `self.CastLightningTimer` _returnvalue)
  (`self.PlaySoundThunder` (`/Game/SkyConstruct/Blueprints/Thunder/BP_Thunder.StrikeLocation` (`self.BP_Thunder`)) (`/Game/SkyConstruct/Blueprints/Thunder/BP_Thunder.CalcMaxStrikeDistance` (`self.BP_Thunder`))))

(event `self.S_ThunderStrikeFar.OnAudioFinished`
  (`self.K2_DestroyActor` :!label _label))

(event `self.S_ThunderStrikeVeryFar.OnAudioFinished`
  (goto _label))

(event `self.S_ThunderStrikeNear.OnAudioFinished`
  (goto _label))

(fn `CastLightning`
  (`ActorComponent.Activate` (`self.ThunderParticle`) false)
  (if (`KismetSystemLibrary.K2_IsTimerActiveHandle` (`self.StopCastLightningTimer`))
    (return)
    (else
      (bind _returnvalue (`KismetSystemLibrary.K2_SetTimer` null "StopCastLightning" (`KismetMathLibrary.RandomFloatInRange` (`self.DelayMinStopCastLightning`) (`self.DelayMaxStopCastLightning`))))
      (set `self.StopCastLightningTimer` _returnvalue)
      (return))))

(fn `CheckReferences`
  (returns (IsValid :type Boolean))
  (return (`KismetSystemLibrary.IsValid` (`self.BP_Thunder`))))

(fn `MaterialFunctionality`
  (`ParticleSystemComponent.SetTemplate` (`self.ThunderParticle`) (`|GetArrayItem` (`self.LightingBoltsParticles`) (`KismetMathLibrary.RandomIntegerInRange` 0 (`KismetArrayLibrary.Array_LastIndex` (`self.LightingBoltsParticles`)))))
  (`PrimitiveComponent.SetMaterial` (`self.ThunderParticle`) 0 (`|GetArrayItem` (`self.LightingMaterials`) (`KismetMathLibrary.RandomIntegerInRange` 0 (`KismetArrayLibrary.Array_LastIndex` (`self.LightingMaterials`))))))

(fn `PlaySoundFar`
  (`AudioComponent.Play` (`self.S_ThunderStrikeFar`) 0.0))

(fn `PlaySoundThunder`
  (params (StrikeLocation_ :type "Vector Structure") (MaxStrikeDistance_ :type "Float (double-precision)"))
  (locals (DistanceToPawnLoc :type "Float (double-precision)" :default 0.0) (DistanceToPawn1Loc :type "Float (double-precision)" :default 0.0))
  (set `local.DistanceToPawnLoc` (`KismetMathLibrary.VSize` (- StrikeLocation_ (`self.K2_GetActorLocation` (`GameplayStatics.GetPlayerPawn` 0)))))
  ;[0 0.3203 1] Сравнить дистанцию с одной третьей от максимальной, двумя третьими и максимальной.
  (set `local.DistanceToPawn1Loc` (/ MaxStrikeDistance_ 3.0))
  (if (`KismetMathLibrary.InRange_FloatFloat` (`local.DistanceToPawnLoc`) 0.0 (`local.DistanceToPawn1Loc`))
    (`AudioComponent.Play` (`self.S_ThunderStrikeNear`) 0.0)
    (elif (`KismetMathLibrary.InRange_FloatFloat` (`local.DistanceToPawnLoc`) (+ (`local.DistanceToPawn1Loc`) 1.0) (* (`local.DistanceToPawn1Loc`) 2.0))
      (`KismetSystemLibrary.K2_SetTimer` null "PlaySoundFar" (`self.DelayPlaySoundFar`))
      (else
        (`KismetSystemLibrary.K2_SetTimer` null "PlaySoundVeryFar" (`self.DelayPlaySoundVeryFar`)))))
  (return))

(fn `PlaySoundVeryFar`
  (`AudioComponent.Play` (`self.S_ThunderStrikeVeryFar`) 0.0))

(fn `StopCastLightning`
  (`KismetSystemLibrary.K2_ClearAndInvalidateTimerHandle` (`self.CastLightningTimer`))
  (`KismetSystemLibrary.K2_ClearAndInvalidateTimerHandle` (`self.StopCastLightningTimer`))
  (`ActorComponent.Deactivate` (`self.ThunderParticle`)))

(fn `UserConstructionScript`)