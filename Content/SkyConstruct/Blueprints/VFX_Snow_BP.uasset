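; Snow weather VFX actor that drives a snow particle component from exposed spawn rate, flake size and force settings.
; SnowFunctionality pushes these to the component as named parameters, randomizing flake size per axis between small and large limits and scaling forces by a random factor.
; It runs from the construction script and again every Tick, so flake size and forces are re-rolled each frame.
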(event `self.ReceiveTick`
  (params (DeltaSeconds :type "Float (single-precision)"))
  (`self.SnowFunctionality`))

(fn `SnowFunctionality`
  (bind _returnvalue (`KismetMathLibrary.RandomFloatInRange` (`self.FlakeSizeSmall`) (`self.FlakeSizeLarge`)))
  (`ParticleSystemComponent.SetFloatParameter` (`self.VFX_Weather_Snow_ForBP`) "SpawnRate" (`self.SpawnRate`))
  (`ParticleSystemComponent.SetVectorParameter` (`self.VFX_Weather_Snow_ForBP`) "FlakeSize" (`KismetMathLibrary.MakeVector` _returnvalue _returnvalue _returnvalue))
  (`ParticleSystemComponent.SetVectorParameter` (`self.VFX_Weather_Snow_ForBP`) "Forces" (* (`self.Forces`) (`KismetMathLibrary.RandomFloatInRange` 0.5 1.5))))

(fn `UserConstructionScript`
  (`self.SnowFunctionality`))